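; BP_Mantis is the playable Mantis hero character, with look, movement, jump and projectile shooting through Enhanced Input.
; BeginPlay initializes ammo, creates the hero HUD and adds the Mantis mapping context.
; Each primary click fires once: a camera trace picks the aim point, and a projectile spawns at the right hand facing it.
; Firing decrements ammo without checking for empty, and the trace draws persistent debug lines.
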(event Input|EnhancedActionEvents|EnhancedInputActionIA_Primary_Click
  (params (ActionValue :type Boolean) (ElapsedSeconds :type Float%20%28double-precision%29) (TriggeredSeconds :type Float%20%28double-precision%29) (InputAction :type Input%20Action%20Object%20Reference :default "/Game/Personnage/Cyril_Mantis/Input/IA_Primary_Click.IA_Primary_Click"))
  (bind _camera (Variables|Default|GetCamera))
  (bind _mesh (Variables|Character|GetMesh))
  (bind _returnvalue (Transformation|GetWorldLocation _camera))
  (bind _returnvalue_2 (Transformation|GetSocketLocation _mesh "hand_r"))
  (:Started
    (Utilities|FlowControl|DoOnce false :!label _label
      (:Completed
        (Math|Integer|DecrementInt (Variables|Default|GetMunitions)
          (:%20%20
            (bind (_outhit _returnvalue_3) (Collision|LineTraceByChannel _returnvalue (+ _returnvalue (* (Math|Vector|GetForwardVector _camera) 1e+04)) "TraceTypeQuery1" false 0 "Persistent"))
            (if _returnvalue_3
              _
              (else
                _))
            (Game|SpawnActorfromClass "/Game/Personnage/Cyril_Mantis/BP_Projectile_Mantis.BP_Projectile_Mantis_C" (Math|Transform|MakeTransform _returnvalue_2 (Math|Rotator|FindLookatRotation _returnvalue_2 (Math|Vector|SelectVector (.ImpactPoint (Collision|BreakHitResult _outhit)) (.TraceEnd (Collision|BreakHitResult _outhit)) _returnvalue_3))) "Undefined" "MultiplyWithRoot" 0 0))))))
  (:Completed
    (goto _label Reset)))

(event Input|EnhancedActionEvents|EnhancedInputActionIA_Look_Commun
  (params (ActionValue :type Vector%202D%20Structure) (ElapsedSeconds :type Float%20%28double-precision%29) (TriggeredSeconds :type Float%20%28double-precision%29) (InputAction :type Input%20Action%20Object%20Reference :default "/Game/Personnage/Cyril_Mantis/Input/IA_Look_Commun.IA_Look_Commun"))
  (Pawn|Input|AddControllerYawInput (.x ActionValue))
  (Pawn|Input|AddControllerPitchInput (.y ActionValue)))

(event Input|EnhancedActionEvents|EnhancedInputActionIA_Move_Commun
  (params (ActionValue :type Vector%202D%20Structure) (ElapsedSeconds :type Float%20%28double-precision%29) (TriggeredSeconds :type Float%20%28double-precision%29) (InputAction :type Input%20Action%20Object%20Reference :default "/Game/Personnage/Cyril_Mantis/Input/IA_Move_Commun.IA_Move_Commun"))
  (bind _returnvalue (Pawn|GetControlRotation :!class /Script/Engine.Pawn))
  (Pawn|Input|AddMovementInput (Math|Vector|GetRightVector (Math|Rotator|MakeRotator (.roll _returnvalue) 0.0 (.yaw _returnvalue))) (.x ActionValue) false)
  (Pawn|Input|AddMovementInput (Math|Vector|GetForwardVector (Math|Rotator|MakeRotator 0.0 0.0 (.yaw (Pawn|GetControlRotation :!class /Script/Engine.Pawn)))) (.y ActionValue) false))

(event Input|EnhancedActionEvents|EnhancedInputActionIA_Jump_Commun
  (params (ActionValue :type Boolean) (ElapsedSeconds :type Float%20%28double-precision%29) (TriggeredSeconds :type Float%20%28double-precision%29) (InputAction :type Input%20Action%20Object%20Reference :default "/Game/Personnage/Cyril_Mantis/Input/IA_Jump_Commun.IA_Jump_Commun"))
  (:Started
    (Character|Jump))
  (:Completed
    (Character|StopJumping)))

(event EventBeginPlay
  (Variables|Default|SetMunitions 20)
  (bind _returnvalue (UserInterface|CreateWidget "/Game/Personnage/Cyril_Mantis/Widget/Wbp_BaseHeroUi_Cyril.Wbp_BaseHeroUi_Cyril_C" 0 self))
  (Variables|Default|SetWidget%20ref _returnvalue)
  (UserInterface|Viewport|AddtoViewport _returnvalue 0)
  (bind _asbp_mantis_controller (Utilities|Casting|CastToBP_Mantis_Controller (Pawn|GetController)))
  (Utilities|IsValid (PlayerController|LocalPlayerSubsystems|GetEnhancedInputLocalPlayerSubsystem _asbp_mantis_controller)
    (:Is%20Valid
      (Input|AddMappingContext (PlayerController|LocalPlayerSubsystems|GetEnhancedInputLocalPlayerSubsystem _asbp_mantis_controller) "/Game/Personnage/Cyril_Mantis/Input/IMC_Mantis.IMC_Mantis" 0 "(bIgnoreAllPressedKeysUntilRelease=True,bForceImmediately=False,bNotifyUserSettings=False)"))))

(fn ConstructionScript)