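; BP_Arrow is a projectile arrow that damages characters it hits, with a Triple variant that explodes.
; Charge sets its speed in the construction script and scales its impact damage, which is fixed for Triple arrows.
; Sphere overlaps ignore the instigator and other arrows, then destroy the arrow or trigger the explosion.
; The explosion, also triggered on projectile stop, damages characters through a sphere trace with persistent debug drawing.
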(event OnComponentBeginOverlap(Sphere)
  (params (OverlappedComponent :type Primitive%20Component%20Object%20Reference) (OtherActor :type Actor%20Object%20Reference) (OtherComp :type Primitive%20Component%20Object%20Reference) (OtherBodyIndex :type Integer) (bFromSweep :type Boolean) (SweepResult :type Hit%20Result%20Structure%20%28by%20ref%29))
  (if (!= (Game|GetInstigator) OtherActor)
    (bind _ascharacter (Utilities|Casting|CastToCharacter OtherActor)
      (:then
        (Game|Damage|ApplyDamage _ascharacter (select (Variables|Default|GetTriple?) 15.0 (Math|Conversions|ToFloat(Integer) (Math|Float|Round (Math|Float|MapRangeClamped (Variables|Default|GetCharge) 0.0 1e+02 1.2e+02 1.8e+02)))) 0 0))
      (:CastFailed
        (Utilities|Casting|CastToBP_Arrow OtherActor
          (:CastFailed
            _))))
    (if (Variables|Default|GetTriple?)
      (CallFunction|Explose)
      (else
        (Actor|DestroyActor)))))

(event OnProjectileStop(ProjectileMovement)
  (params (ImpactResult :type Hit%20Result%20Structure%20%28by%20ref%29))
  (bind _hitactor (Collision|BreakHitResult ImpactResult))
  (if (and (not (or (== _hitactor (Game|GetInstigator)) (== _hitactor "BP_Arrow"))) (Variables|Default|GetTriple?))
    (CallFunction|Explose)))

(event Custom|Explose
  (bind _sphere (Variables|Default|GetSphere))
  (bind _returnvalue (Transformation|GetWorldLocation _sphere))
  (bind _outhits (Collision|MultiSphereTraceByChannel _returnvalue _returnvalue 3e+02 "TraceTypeQuery1" false 0 "Persistent"))
  (for _array_element _outhits
    (bind _ascharacter (Utilities|Casting|CastToCharacter (.HitActor (Collision|BreakHitResult _array_element))))
    (Game|Damage|ApplyDamage _ascharacter 32.0 0 0))
  (Actor|DestroyActor))

(event EventBeginPlay)

(fn ConstructionScript
  (bind _projectilemovement (Variables|Default|GetProjectileMovement))
  (bind _charge (Variables|Default|GetCharge))
  (bind _returnvalue (Math|Float|MapRangeClamped _charge 0.0 1e+02 5.2e+03 1e+04))
  (Variables|/Script/Engine.ProjectileMovementComponent|SetInitialSpeed _projectilemovement _returnvalue)
  (Variables|/Script/Engine.ProjectileMovementComponent|SetMaxSpeed _projectilemovement _returnvalue))