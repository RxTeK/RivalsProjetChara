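; Actor component that gives the HawkEye character Skyward Leap, a directional double jump usable while falling.
; Jump input zeroes velocity, then launches the owner upward and along the stored move input relative to facing, defaulting to forward.
; A looping timer at frame-delta interval polls for landing, then starts the cooldown that re-enables the leap.
; Debug prints show move input every tick and the launch vector.
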(event Custom|Isfalling
  (if (AI|Components|NavMovement|IsMovingonGround (Variables|/Script/Engine.Character|GetCharacterMovement (Variables|Default|GetPlayer_Ref)))
    (Utilities|Time|ClearandInvalidateTimerbyHandle (Variables|Default|GetTicked))
    (Utilities|Time|SetTimerbyEvent (delegate Custom|CD_DoubleJump) 6.0)))

(event Custom|CD_DoubleJump
  (Variables|Default|SetDoubleJump? false))

(event Input|EnhancedActionEvents|EnhancedInputActionIA_MoveHawk
  (params (ActionValue :type Vector%202D%20Structure) (ElapsedSeconds :type Float%20%28double-precision%29) (TriggeredSeconds :type Float%20%28double-precision%29) (InputAction :type Input%20Action%20Object%20Reference :default "/Game/Personnage/MaximeHawkEye/Input/InputAction/IA_MoveHawk.IA_MoveHawk"))
  (:Triggered
    (Variables|Default|SetAction%20Value ActionValue))
  (:Completed
    (Variables|Default|SetAction%20Value "")))

(event Input|EnhancedActionEvents|EnhancedInputActionIA_JumpHawk
  (params (ActionValue :type Boolean) (ElapsedSeconds :type Float%20%28double-precision%29) (TriggeredSeconds :type Float%20%28double-precision%29) (InputAction :type Input%20Action%20Object%20Reference :default "/Game/Personnage/MaximeHawkEye/Input/InputAction/IA_JumpHawk.IA_JumpHawk"))
  (bind _player_ref (Variables|Default|GetPlayer_Ref))
  (bind _player_ref_2 (Variables|Default|GetPlayer_Ref))
  (bind _action_value (Variables|Default|GetAction%20Value))
  (bind _returnvalue (Transformation|GetActorForwardVector _player_ref_2))
  (bind _returnvalue_2 (Transformation|GetActorRightVector _player_ref))
  (bind _returnvalue_3 (Transformation|GetActorForwardVector _player_ref))
  (bind _returnvalue_4 (* (.x _action_value) _returnvalue_3))
  (bind _returnvalue_5 (* (.y _action_value) _returnvalue_2))
  (bind _returnvalue_6 (+ _returnvalue_4 _returnvalue_5))
  (bind _returnvalue_7 (Math|Vector|Normalize _returnvalue_6))
  (bind (_x _y) (Math|Vector|BreakVector _returnvalue_6))
  (bind _returnvalue_8 (== _x 0.0))
  (bind _returnvalue_9 (== _y 0.0))
  (bind _returnvalue_10 (and _returnvalue_8 _returnvalue_9))
  (bind _returnvalue_11 (select _returnvalue_10 _returnvalue _returnvalue_7))
  (bind _returnvalue_12 (* _returnvalue_11 1.2e+03))
  (bind _returnvalue_13 (+ _returnvalue_12 "0.000000,0.000000,1200.000000"))
  (:Started
    (Development|PrintString "Hello")
    (if (and (AI|Components|NavMovement|IsFalling (Variables|/Script/Engine.Character|GetCharacterMovement (Variables|Default|GetPlayer_Ref))) (not (Variables|Default|GetDoubleJump?)))
      (Variables|Default|SetDoubleJump? true)
      (bind _returnvalue_14 (Utilities|Time|SetTimerbyEvent (delegate Custom|Isfalling) (Utilities|Time|GetWorldDeltaSeconds) true))
      (Variables|Default|SetTicked _returnvalue_14)
      (Variables|/Script/Engine.MovementComponent|SetVelocity (Variables|/Script/Engine.Character|GetCharacterMovement (Variables|Default|GetPlayer_Ref)) "0, 0, 0")
      (Development|PrintString (Utilities|String|ToString(Vector) _returnvalue_13))
      (Character|LaunchCharacter (Variables|Default|GetPlayer_Ref) _returnvalue_13 false false))))

(event EventBeginPlay
  (bind _ascharacter (Utilities|Casting|CastToCharacter (Components|GetOwner)))
  (Variables|Default|SetPlayer_Ref _ascharacter))

(event EventTick
  (params (DeltaSeconds :type Float%20%28single-precision%29))
  (Development|PrintString (Utilities|String|ToString(Vector2d) (Variables|Default|GetAction%20Value)) true true "(R=0.000000,G=0.660000,B=1.000000,A=1.000000)" 0.0))