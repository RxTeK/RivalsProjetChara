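; Hawkeye's second ability, owned by BP_Player, which fires a hypersonic arrow followed by a delayed damage sweep.
; Input plays the shot montage, whose notify traces from the camera and then the bow's shoot point to aim and spawn BP_ArrowHypersonic.
; Half a second later, a wide capsule trace along the saved line damages each Character once.
; Montage completion or interruption starts the cooldown, gated by timer handle validity.
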(event Custom|Second
  (bind _locatestart (Variables|Default|GetLocateStart))
  (bind _outhits (Class|KismetSystemLibrary|CapsuleTraceMultiforObjects _locatestart (+ (* (Variables|Default|GetSecondCastExplosion) (Variables|Default|GetLenght)) _locatestart) 3e+02 0.0 (Utilities|Array|MakeArray "ObjectTypeQuery3") false 0 "ForDuration" true))
  (for _array_element _outhits
    (bind _ascharacter (Utilities|Casting|CastToCharacter (.HitActor (Collision|BreakHitResult _array_element))))
    (if (== (Utilities|Array|FindItem (Variables|Default|GetTouch) _ascharacter) -1)
      (Utilities|Array|AddUnique (Variables|Default|GetTouch) _ascharacter)
      (Game|Damage|ApplyDamage _ascharacter 5e+01 0 0)))
  (Utilities|Array|Clear (Variables|Default|GetTouch)))

(event Custom|InCD
  (Utilities|Time|ClearandInvalidateTimerbyHandle (Variables|Default|GetNewVar_0)))

(event Input|EnhancedActionEvents|EnhancedInputActionIA_SecondAbilityHawk
  (params (ActionValue :type Boolean) (ElapsedSeconds :type Float%20%28double-precision%29) (TriggeredSeconds :type Float%20%28double-precision%29) (InputAction :type Input%20Action%20Object%20Reference :default "/Game/Personnage/MaximeHawkEye/Input/InputAction/IA_SecondAbilityHawk.IA_SecondAbilityHawk"))
  (bind _hawk_ref (Variables|Default|GetHawk_Ref))
  (bind _hawk_ref_2 (Variables|Default|GetHawk_Ref))
  (bind _hawk_ref_3 (Variables|Default|GetHawk_Ref))
  (bind _lenght (Variables|Default|GetLenght))
  (bind _shootimplace (Variables|/Game/Personnage/ALL/BP_Player.BP_Player_C|GetShootImplace _hawk_ref))
  (bind _followcamera (Variables|/Game/Personnage/ALL/BP_Player.BP_Player_C|GetFollowCamera _hawk_ref_3))
  (bind _shootimplace_2 (Variables|/Game/Personnage/ALL/BP_Player.BP_Player_C|GetShootImplace _hawk_ref_2))
  (bind _returnvalue (Transformation|GetWorldLocation _followcamera))
  (bind _returnvalue_2 (Transformation|GetWorldLocation _shootimplace))
  (bind _returnvalue_3 (Transformation|GetWorldLocation _shootimplace_2))
  (bind _returnvalue_4 (Math|Vector|GetForwardVector _followcamera))
  (bind _returnvalue_5 (* _returnvalue_4 _lenght))
  (:Started
    (if (not (Utilities|Time|IsValidTimerHandle (Variables|Default|GetNewVar_0)))
      (Variables|Default|SetTrue true)
      (Animation|Montage|PlayMontage (Variables|/Script/Engine.Character|GetMesh (Variables|Default|GetHawk_Ref)) "/Game/Personnage/MaximeHawkEye/Animation/Anim/HEyeAnim_SK_1021_1021001_102161_Competance.HEyeAnim_SK_1021_1021001_102161_Competance" 1.0 0.0 "Arrow"
        (:OnCompleted
          (bind _returnvalue_6 (Utilities|Time|SetTimerbyEvent (delegate Custom|InCD) 12.0 :!label _label))
          (Variables|Default|SetNewVar_0 _returnvalue_6)
          (Variables|Default|SetTrue false))
        (:OnInterrupted
          (goto _label))
        (:OnNotifyBegin
          (bind (_outhit _returnvalue_7) (Collision|LineTraceForObjects _returnvalue (+ _returnvalue _returnvalue_5) (Utilities|Array|MakeArray "ObjectTypeQuery1" "ObjectTypeQuery3") false 0 "ForDuration" true "(R=0.053799,G=1.000000,B=0.000000,A=1.000000)"))
          (Variables|Default|SetLocateStart _returnvalue_2)
          (bind (_outhit_2 _returnvalue_8) (Collision|LineTraceForObjects (Transformation|GetWorldLocation (Variables|/Game/Personnage/ALL/BP_Player.BP_Player_C|GetShootImplace (Variables|Default|GetHawk_Ref))) (select _returnvalue_7 (select (> (Math|Vector|DotProduct (Math|Vector|GetUnitDirection(Vector) _returnvalue_2 (.Location (Collision|BreakHitResult _outhit))) (Math|Vector|GetForwardVector (Variables|/Game/Personnage/ALL/BP_Player.BP_Player_C|GetFollowCamera (Variables|Default|GetHawk_Ref)))) 0.9) (.Location (Collision|BreakHitResult _outhit)) _returnvalue_5) (.TraceEnd (Collision|BreakHitResult _outhit))) (Utilities|Array|MakeArray "ObjectTypeQuery1" "ObjectTypeQuery3") false 0 "ForDuration" true "(R=1.000000,G=0.000000,B=0.797801,A=1.000000)"))
          (Variables|Default|SetSecondCastExplosion (Math|Vector|GetUnitDirection(Vector) _returnvalue_3 (select _returnvalue_8 (.Location (Collision|BreakHitResult _outhit_2)) (.TraceEnd (Collision|BreakHitResult _outhit_2)))))
          (Game|SpawnActorfromClass "/Game/Personnage/MaximeHawkEye/Blueprint/BP_ArrowHypersonic.BP_ArrowHypersonic_C" (Math|Transform|MakeTransform _returnvalue_3 (Math|Rotator|FindLookatRotation _returnvalue_3 (select _returnvalue_8 (.Location (Collision|BreakHitResult _outhit_2)) (.TraceEnd (Collision|BreakHitResult _outhit_2)))) "1.000000,1.000000,1.000000") "Undefined" "MultiplyWithRoot" 0 0.0 0.0 false (Variables|Default|GetHawk_Ref))
          (Utilities|Time|SetTimerbyEvent (delegate Custom|Second) 0.5))))))

(event EventBeginPlay
  (bind _asbp_player (Utilities|Casting|CastToBP_Player (Components|GetOwner)))
  (Variables|Default|SetHawk_Ref _asbp_player))