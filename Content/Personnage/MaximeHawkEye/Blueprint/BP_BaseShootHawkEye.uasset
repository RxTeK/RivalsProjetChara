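; Hawkeye's bow shooting component for BP_Player, switching between single arrows and an ammo-limited three-arrow spread, and updating the HUD.
; Holding fire slows movement and builds charge; release, buffered until the draw montage finishes, spawns BP_Arrow with that charge.
; Aim traces from the camera, then from the bow socket, with a dot-product check against skewed angles.
; Timers drive ammo reload, weapon-swap delay and the return to neutral state.
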(event Custom|ReShoot
  (Variables|Default|SetDelay true))

(event Custom|Triple
  (if (Variables|Default|GetTriple?)
    (bind _output_get (Variables|Default|SetMunitions (Math|Float|Clamp(Float) (- (Variables|Default|GetMunitions) 1.0) 0.0 3.0)))
    (Default|SetMunitions (Variables|/Game/Personnage/ALL/BP_Player.BP_Player_C|GetHUD%20REF (Variables|Default|GetHawk_Ref)) _output_get 3.0)
    (if (not (Utilities|Time|IsValidTimerHandle (Variables|Default|GetNewVar)))
      (bind _returnvalue (Utilities|Time|SetTimerbyEvent (delegate Custom|Reload) 3.0 true))
      (Variables|Default|SetNewVar _returnvalue))))

(event Custom|Reload
  (bind _output_get (Variables|Default|SetMunitions (Math|Float|Clamp(Float) (+ (Variables|Default|GetMunitions) 1.0) 0.0 3.0)))
  (if (Variables|Default|GetTriple?)
    (Default|SetMunitions (Variables|/Game/Personnage/ALL/BP_Player.BP_Player_C|GetHUD%20REF (Variables|Default|GetHawk_Ref)) _output_get 3.0))
  (if (>= (Variables|Default|GetMunitions) 3.0)
    (Utilities|Time|ClearandInvalidateTimerbyHandle (Variables|Default|GetNewVar))))

(event Custom|ShootArrow
  (params (Triple :type Boolean))
  (bind _hawk_ref (Variables|Default|GetHawk_Ref))
  (bind _hawk_ref_2 (Variables|Default|GetHawk_Ref))
  (bind _followcamera (Variables|/Game/Personnage/ALL/BP_Player.BP_Player_C|GetFollowCamera _hawk_ref))
  (bind _shootimplace (Variables|/Game/Personnage/ALL/BP_Player.BP_Player_C|GetShootImplace _hawk_ref_2))
  (bind _returnvalue (Transformation|GetWorldLocation _followcamera))
  (bind _returnvalue_2 (Transformation|GetWorldLocation _shootimplace))
  (bind _returnvalue_3 (Math|Vector|GetForwardVector _followcamera))
  (Utilities|Time|ClearandInvalidateTimerbyHandle (Variables|Default|GetChargeArrowTH))
  (for _index (range 0 (select Triple 2 0))
    (Variables|Default|SetIndex _index)
    (bind (_outhit _returnvalue_4) (Collision|LineTraceForObjects _returnvalue (+ _returnvalue (* (Utilities|Select :Index (Variables|Default|GetIndex) :Option%200 _returnvalue_3 :Option%201 (Math|Vector|RotateVector _returnvalue_3 "0.000000,10.000000,0.000000") :Option%202 (Math|Vector|RotateVector _returnvalue_3 "0.000000,-10.000000,0.000000")) 4e+03)) (Utilities|Array|MakeArray "ObjectTypeQuery1" "ObjectTypeQuery3") false 0 "ForDuration"))
    (bind (_outhit_2 _returnvalue_5) (Collision|LineTraceForObjects (Transformation|GetWorldLocation (Variables|/Game/Personnage/ALL/BP_Player.BP_Player_C|GetShootImplace (Variables|Default|GetHawk_Ref))) (select _returnvalue_4 (select (> (Math|Vector|DotProduct (Math|Vector|GetUnitDirection(Vector) (Transformation|GetWorldLocation (Variables|/Game/Personnage/ALL/BP_Player.BP_Player_C|GetShootImplace (Variables|Default|GetHawk_Ref))) (.Location (Collision|BreakHitResult _outhit))) (Math|Vector|GetForwardVector (Variables|/Game/Personnage/ALL/BP_Player.BP_Player_C|GetFollowCamera (Variables|Default|GetHawk_Ref)))) (select (> (Variables|Default|GetIndex) 0) 0.7 0.9)) (.Location (Collision|BreakHitResult _outhit)) (* (Utilities|Select :Index (Variables|Default|GetIndex) :Option%200 _returnvalue_3 :Option%201 (Math|Vector|RotateVector _returnvalue_3 "0.000000,10.000000,0.000000") :Option%202 (Math|Vector|RotateVector _returnvalue_3 "0.000000,-10.000000,0.000000")) 4e+03)) (.TraceEnd (Collision|BreakHitResult _outhit))) (Utilities|Array|MakeArray "ObjectTypeQuery1" "ObjectTypeQuery3") false 0 "ForDuration"))
    (Game|SpawnActorfromClass "/Game/Personnage/MaximeHawkEye/Blueprint/BP_Arrow.BP_Arrow_C" (Math|Transform|MakeTransform _returnvalue_2 (Math|Rotator|FindLookatRotation _returnvalue_2 (select _returnvalue_5 (.Location (Collision|BreakHitResult _outhit_2)) (.TraceEnd (Collision|BreakHitResult _outhit_2)))) "1.000000,1.000000,1.000000") "Undefined" "MultiplyWithRoot" 0 (Variables|Default|GetArrowStrong) 0.0 (Variables|Default|GetTriple?) (Variables|Default|GetHawk_Ref)))
  (Variables|Default|SetArrowStrong 0.0))

(event Custom|Timeer
  (Variables|Default|SetFistAnimFinish false)
  (Utilities|Time|ClearandInvalidateTimerbyHandle (Variables|Default|GetChargeArrowTH))
  (bind _returnvalue (Utilities|Time|SetTimerbyEvent (delegate Custom|To%20Neutral) 1e+01))
  (Variables|Default|SetTime%20To%20no%20combat _returnvalue)
  (CallFunction|ShootArrow (Variables|Default|GetTriple?))
  (CallFunction|Triple)
  (Variables|/Script/Engine.CharacterMovementComponent|SetMaxWalkSpeed (Variables|/Script/Engine.Character|GetCharacterMovement (Variables|Default|GetHawk_Ref)) (Variables|Default|GetMax%20Walk%20Speed))
  (Animation|Montage|PlayMontage (Variables|/Script/Engine.Character|GetMesh (Variables|Default|GetHawk_Ref)) (select (Variables|Default|GetTriple?) "/Game/Personnage/MaximeHawkEye/Animation/Anim/HEyeAnim_SK_1021_1021001_102131_ShootThree_Montage.HEyeAnim_SK_1021_1021001_102131_ShootThree_Montage" "/Game/Personnage/MaximeHawkEye/Animation/Anim/HEyeAnim_SK_1021_1021001_102131_ShootOne_Montage.HEyeAnim_SK_1021_1021001_102131_ShootOne_Montage") 1.0 0.0 (Utilities|Name|MakeLiteralName "End")
    (:OnCompleted
      _)
    (:OnInterrupted
      _))
  (Variables|Default|SetEnumHAWK "NewEnumerator1")
  (Variables|Default|SetInshoot false)
  (if (Variables|Default|GetCouldShoot)
    (CallFunction|ShootSpeed)))

(event Custom|ChargeArrow
  (bind _output_get (Variables|Default|SetArrowStrong (Math|Interpolation|FInterptoConstant (Variables|Default|GetArrowStrong) 1e+02 (Utilities|Time|GetWorldDeltaSeconds) 115.0)))
  (Development|PrintString (Utilities|String|ToString(Float) _output_get) true true "(R=0.000000,G=0.660000,B=1.000000,A=1.000000)" 0.0))

(event Custom|Tim
  (bind _hawk_ref (Variables|Default|GetHawk_Ref))
  (Variables|Default|SetArrowStrong 0.0)
  (Variables|/Game/Personnage/ALL/WBP_HUDScarlet.WBP_HUDScarlet_C|SetTexture%20auto (Variables|/Game/Personnage/ALL/BP_Player.BP_Player_C|GetHUD%20REF _hawk_ref) (select (Variables|Default|GetTriple?) "/Game/Personnage/MaximeHawkEye/Image/b54fcda9-4e31-4a7b-87c7-c7e8fd675434.b54fcda9-4e31-4a7b-87c7-c7e8fd675434" "/Game/Personnage/MaximeHawkEye/Image/9107db4e-f275-49aa-87bf-96c697157a15.9107db4e-f275-49aa-87bf-96c697157a15"))
  (Default|SetComp (Variables|/Game/Personnage/ALL/BP_Player.BP_Player_C|GetHUD%20REF _hawk_ref) "Hidden" "Visible" "Visible" "Visible")
  (if (Variables|Default|GetTriple?)
    (Default|SetMunitions (Variables|/Game/Personnage/ALL/BP_Player.BP_Player_C|GetHUD%20REF (Variables|Default|GetHawk_Ref)) (Variables|Default|GetMunitions) 3.0)
    (else
      (Default|SetMunitions (Variables|/Game/Personnage/ALL/BP_Player.BP_Player_C|GetHUD%20REF (Variables|Default|GetHawk_Ref)) 0.0 0.0)))
  (Utilities|Time|SetTimerbyEvent (delegate Custom|ReShoot) 0.7))

(event Custom|To%20Neutral
  (Variables|Default|SetEnumHAWK "NewEnumerator2"))

(event Custom|ShootSpeed
  (bind _returnvalue (Utilities|Time|GetWorldDeltaSeconds))
  (bind _hawk_ref (Variables|Default|GetHawk_Ref))
  (bind _charactermovement (Variables|/Script/Engine.Character|GetCharacterMovement _hawk_ref))
  (if (Variables|Default|GetTriple?)
    (if (> (Variables|Default|GetMunitions) 0.0)
      (Utilities|Time|ClearandInvalidateTimerbyHandle (Variables|Default|GetTime%20To%20no%20combat) :!label _label)
      (Variables|Default|SetInshoot true)
      (Variables|Default|SetEnumHAWK "NewEnumerator0")
      (bind _returnvalue_2 (Utilities|Time|SetTimerbyEvent (EventDispatchers|CreateEvent :!event Custom|ChargeArrow) _returnvalue true false (* _returnvalue -1.0)))
      (Variables|Default|SetChargeArrowTH _returnvalue_2)
      (Variables|Default|SetMax%20Walk%20Speed (Variables|/Script/Engine.CharacterMovementComponent|GetMaxWalkSpeed _charactermovement))
      (Variables|/Script/Engine.CharacterMovementComponent|SetMaxWalkSpeed _charactermovement (* (Variables|Default|GetMax%20Walk%20Speed) 0.7))
      (Animation|Montage|PlayMontage (Variables|/Script/Engine.Character|GetMesh (Variables|Default|GetHawk_Ref)) (select (Variables|Default|GetTriple?) "/Game/Personnage/MaximeHawkEye/Animation/Anim/HEyeAnim_SK_1021_1021001_102131_DrawThree_Montage.HEyeAnim_SK_1021_1021001_102131_DrawThree_Montage" "/Game/Personnage/MaximeHawkEye/Animation/Anim/HEyeAnim_SK_1021_1021001_102131_DrawOne_Montage.HEyeAnim_SK_1021_1021001_102131_DrawOne_Montage") 1.0 0.0 "Charge"
        (:OnCompleted
          (Variables|Default|SetFistAnimFinish true)
          (if (Variables|Default|GetWouldShoot)
            (CallFunction|Timeer)))))
    (else
      (goto _label))))

(event Input|EnhancedActionEvents|EnhancedInputActionIA_ShootHawk
  (params (ActionValue :type Boolean) (ElapsedSeconds :type Float%20%28double-precision%29) (TriggeredSeconds :type Float%20%28double-precision%29) (InputAction :type Input%20Action%20Object%20Reference :default "/Game/Personnage/MaximeHawkEye/Input/InputAction/IA_ShootHawk.IA_ShootHawk"))
  (bind _returnvalue (Utilities|Time|GetWorldDeltaSeconds))
  (bind _hawk_ref (Variables|Default|GetHawk_Ref))
  (bind _charactermovement (Variables|/Script/Engine.Character|GetCharacterMovement _hawk_ref))
  (:Triggered
    (Variables|Default|SetAction%20Value ActionValue))
  (:Started
    (Variables|Default|SetFistAnimFinish false)
    (Variables|Default|SetWouldShoot false)
    (Variables|Default|SetCouldShoot true)
    (if (not (Variables|Default|GetInshoot))
      (if (Variables|Default|GetTriple?)
        (if (> (Variables|Default|GetMunitions) 0.0)
          (Utilities|Time|ClearandInvalidateTimerbyHandle (Variables|Default|GetTime%20To%20no%20combat) :!label _label)
          (Variables|Default|SetInshoot true)
          (Variables|Default|SetEnumHAWK "NewEnumerator0")
          (bind _returnvalue_2 (Utilities|Time|SetTimerbyEvent (EventDispatchers|CreateEvent :!event Custom|ChargeArrow) _returnvalue true false (* _returnvalue -1.0)))
          (Variables|Default|SetChargeArrowTH _returnvalue_2)
          (Variables|Default|SetMax%20Walk%20Speed (Variables|/Script/Engine.CharacterMovementComponent|GetMaxWalkSpeed _charactermovement))
          (Variables|/Script/Engine.CharacterMovementComponent|SetMaxWalkSpeed _charactermovement (* (Variables|Default|GetMax%20Walk%20Speed) 0.7))
          (Animation|Montage|PlayMontage (Variables|/Script/Engine.Character|GetMesh (Variables|Default|GetHawk_Ref)) (select (Variables|Default|GetTriple?) "/Game/Personnage/MaximeHawkEye/Animation/Anim/HEyeAnim_SK_1021_1021001_102131_DrawThree_Montage.HEyeAnim_SK_1021_1021001_102131_DrawThree_Montage" "/Game/Personnage/MaximeHawkEye/Animation/Anim/HEyeAnim_SK_1021_1021001_102131_DrawOne_Montage.HEyeAnim_SK_1021_1021001_102131_DrawOne_Montage") 1.0 0.0 "Charge"
            (:OnCompleted
              (Variables|Default|SetFistAnimFinish true)
              (if (Variables|Default|GetWouldShoot)
                (CallFunction|Timeer)))))
        (else
          (goto _label)))))
  (:Canceled
    (Variables|Default|SetAction%20Value false :!label _label_2)
    (Variables|Default|SetCouldShoot false)
    (if (Variables|Default|GetFistAnimFinish)
      (if (and (Variables|Default|GetDelay2) (Variables|Default|GetInshoot))
        (CallFunction|Timeer))
      (else
        (Variables|Default|SetWouldShoot true))))
  (:Completed
    (goto _label_2)))

(event Input|EnhancedActionEvents|EnhancedInputActionIA_ChangeWeaponHawk
  (params (ActionValue :type Float%20%28double-precision%29) (ElapsedSeconds :type Float%20%28double-precision%29) (TriggeredSeconds :type Float%20%28double-precision%29) (InputAction :type Input%20Action%20Object%20Reference :default "/Game/Personnage/MaximeHawkEye/Input/InputAction/IA_ChangeWeaponHawk.IA_ChangeWeaponHawk"))
  (:Started
    (if (and (Variables|Default|GetDelay) (not (Variables|Default|GetInshoot)))
      (Variables|Default|SetDelay false)
      (Variables|Default|SetTriple? (not (== ActionValue 1.0)))
      (CallFunction|Tim))))

(event Input|EnhancedActionEvents|EnhancedInputActionIA_ChangeWeaponRollHawk
  (params (ActionValue :type Float%20%28double-precision%29) (ElapsedSeconds :type Float%20%28double-precision%29) (TriggeredSeconds :type Float%20%28double-precision%29) (InputAction :type Input%20Action%20Object%20Reference :default "/Game/Personnage/MaximeHawkEye/Input/InputAction/IA_ChangeWeaponRollHawk.IA_ChangeWeaponRollHawk"))
  (if (and (Variables|Default|GetDelay) (not (Variables|Default|GetInshoot)))
    (Variables|Default|SetDelay false)
    (Variables|Default|SetTriple? (not (Variables|Default|GetTriple?)))
    (CallFunction|Tim)))

(event EventTick
  (params (DeltaSeconds :type Float%20%28single-precision%29))
  (Development|PrintString (Utilities|String|Append "etat" " == " (Utilities|String|EnumtoString (Variables|Default|GetEnumHAWK))) true true "(R=0.000000,G=0.660000,B=1.000000,A=1.000000)" 0.0))

(event EventBeginPlay
  (bind _asbp_player (Utilities|Casting|CastToBP_Player (Components|GetOwner)))
  (Variables|Default|SetHawk_Ref _asbp_player)
  (Variables|/Game/Personnage/ALL/WBP_HUDScarlet.WBP_HUDScarlet_C|SetComp%203 (Variables|/Game/Personnage/ALL/BP_Player.BP_Player_C|GetHUD%20REF (Variables|Default|GetHawk_Ref)) "Shift")
  (Variables|/Game/Personnage/ALL/WBP_HUDScarlet.WBP_HUDScarlet_C|SetComp%204 (Variables|/Game/Personnage/ALL/BP_Player.BP_Player_C|GetHUD%20REF (Variables|Default|GetHawk_Ref)) "E")
  (Variables|/Game/Personnage/ALL/WBP_HUDScarlet.WBP_HUDScarlet_C|SetComp%202 (Variables|/Game/Personnage/ALL/BP_Player.BP_Player_C|GetHUD%20REF (Variables|Default|GetHawk_Ref)) "Space")
  (Variables|/Game/Personnage/ALL/WBP_HUDScarlet.WBP_HUDScarlet_C|SetTexture%20Perso (Variables|/Game/Personnage/ALL/BP_Player.BP_Player_C|GetHUD%20REF (Variables|Default|GetHawk_Ref)) "/Game/Personnage/MaximeHawkEye/Image/d27.d27")
  (Variables|/Game/Personnage/ALL/WBP_HUDScarlet.WBP_HUDScarlet_C|SetTexture%20auto (Variables|/Game/Personnage/ALL/BP_Player.BP_Player_C|GetHUD%20REF (Variables|Default|GetHawk_Ref)) "/Game/Personnage/MaximeHawkEye/Image/9107db4e-f275-49aa-87bf-96c697157a15.9107db4e-f275-49aa-87bf-96c697157a15")
  (Variables|/Game/Personnage/ALL/WBP_HUDScarlet.WBP_HUDScarlet_C|SetTexture%20Comp%202 (Variables|/Game/Personnage/ALL/BP_Player.BP_Player_C|GetHUD%20REF (Variables|Default|GetHawk_Ref)) "/Game/Personnage/MaximeHawkEye/Image/83892ce1-2db5-4c6c-a0f2-a4117ab86aab.83892ce1-2db5-4c6c-a0f2-a4117ab86aab")
  (Variables|/Game/Personnage/ALL/WBP_HUDScarlet.WBP_HUDScarlet_C|SetTexture%20comp%203 (Variables|/Game/Personnage/ALL/BP_Player.BP_Player_C|GetHUD%20REF (Variables|Default|GetHawk_Ref)) "/Game/Personnage/MaximeHawkEye/Image/a598cd3c-e1d2-4403-8d48-13bf9dcf1b39.a598cd3c-e1d2-4403-8d48-13bf9dcf1b39")
  (Variables|/Game/Personnage/ALL/WBP_HUDScarlet.WBP_HUDScarlet_C|SetTexture%20comp%204 (Variables|/Game/Personnage/ALL/BP_Player.BP_Player_C|GetHUD%20REF (Variables|Default|GetHawk_Ref)) "/Game/Personnage/MaximeHawkEye/Image/96e35f6b-b42a-461a-9cd9-554ed05e3470.96e35f6b-b42a-461a-9cd9-554ed05e3470")
  (Default|SetComp (Variables|/Game/Personnage/ALL/BP_Player.BP_Player_C|GetHUD%20REF (Variables|Default|GetHawk_Ref)) "Hidden" "Visible" "Visible" "Visible"))