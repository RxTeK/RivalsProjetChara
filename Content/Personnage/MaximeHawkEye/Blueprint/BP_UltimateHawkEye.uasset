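; Hawk Eye ultimate ability that periodically leaves afterimages (BP_Remanente) on every BP_Dummy for a limited duration.
; The IA_UltimateHawk input starts a looping timer unless one is already running.
; Each tick of that timer spawns an afterimage at each dummy's transform, passing its mesh to copy and the dummy as damage owner.
; The timer clears itself once accumulated time exceeds TimeToEnd.
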(event Custom|SpawnRemanante
  (Variables|Default|SetTimeIn (+ (Variables|Default|GetTime) (Variables|Default|GetTimeIn)))
  (if (>= (Variables|Default|GetTimeToEnd) (Variables|Default|GetTimeIn))
    (bind _outactors (Actor|GetAllActorsOfClass "/Game/Personnage/Dummy/BP_Dummy.BP_Dummy_C"))
    (for _array_element _outactors
      (Game|SpawnActorfromClass "/Game/Personnage/MaximeHawkEye/Blueprint/BP_Remanente.BP_Remanente_C" (Transformation|GetActorTransform _array_element) "Undefined" "MultiplyWithRoot" 0 (Variables|/Script/Engine.Character|GetMesh _array_element) _array_element 0))
    (else
      (Utilities|Time|ClearandInvalidateTimerbyHandle (Variables|Default|GetValue)))))

(event Input|EnhancedActionEvents|EnhancedInputActionIA_UltimateHawk
  (params (ActionValue :type Boolean) (ElapsedSeconds :type Float%20%28double-precision%29) (TriggeredSeconds :type Float%20%28double-precision%29) (InputAction :type Input%20Action%20Object%20Reference :default "/Game/Personnage/MaximeHawkEye/Input/InputAction/IA_UltimateHawk.IA_UltimateHawk"))
  (:Started
    (if (not (Utilities|Time|IsValidTimerHandle (Variables|Default|GetValue)))
      (Variables|Default|SetTimeIn 0.0)
      (bind _returnvalue (Utilities|Time|SetTimerbyEvent (delegate Custom|SpawnRemanante) (Variables|Default|GetTime) true))
      (Variables|Default|SetValue _returnvalue))))

(event EventBeginPlay)

(event EventTick
  (params (DeltaSeconds :type Float%20%28single-precision%29)))