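; Zipline actor for the Punisher character, built as a two-point spline to EndPos with a spline mesh generated in the construction script.
; Once player 0 passes the start on Y, Tick snaps a trigger box to the spline, tracking the player's Y or advancing at SpeedOnZipline while attached.
; Overlapping the box attaches the player if CanAttach is true.
; Near the end, it detaches any rider and destroys the box.
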(event OnComponentBeginOverlap(BoxP1)
  (params (OverlappedComponent :type Primitive%20Component%20Object%20Reference) (OtherActor :type Actor%20Object%20Reference) (OtherComp :type Primitive%20Component%20Object%20Reference) (OtherBodyIndex :type Integer) (bFromSweep :type Boolean) (SweepResult :type Hit%20Result%20Structure%20%28by%20ref%29))
  (bind _returnvalue (Game|GetPlayerCharacter 0))
  (if (== OtherActor _returnvalue)
    (bind _asbp_punisher (Utilities|Casting|CastToBP_Punisher _returnvalue))
    (if (Variables|/Game/Personnage/PunisherNelson/Bp/BP_Punisher.BP_Punisher_C|GetCanAttach _asbp_punisher)
      (Default|ManageZipline _asbp_punisher true)
      (Variables|/Game/Personnage/PunisherNelson/Bp/BP_Punisher.BP_Punisher_C|SetZiplineRef _asbp_punisher self))))

(event EventBeginPlay)

(event Collision|EventActorBeginOverlap
  (params (OtherActor :type Actor%20Object%20Reference)))

(event EventTick
  (params (DeltaSeconds :type Float%20%28single-precision%29))
  (Utilities|FlowControl|Sequence
    (:then_0
      (bind _isactive (CallFunction|SplineActive))
      (if _isactive
        (Variables|Default|GetBoxP1
          (:then
            (CallFunction|BoxMovement))
          (:else))))))

(fn ConstructionScript
  (bind _spline (Variables|Default|GetSpline))
  (Spline|SetLocationatSplinePoint (Variables|Default|GetSpline) 1 (Variables|Default|GetEnd%20Pos) "World" true)
  (bind _returnvalue (AddComponent|AddSplineMeshComponent false))
  (SplineMesh|SetForwardAxis _returnvalue "X" true)
  (SplineMesh|SetStartandEnd _returnvalue (Spline|GetLocationatSplinePoint _spline 0 "Local") (Spline|GetTangentatSplinePoint _spline 0 "Local") (Spline|GetLocationatSplinePoint _spline 1 "Local") (Spline|GetTangentatSplinePoint _spline 1 "Local") true :!class /Script/Engine.SplineMeshComponent))

(fn SplineActive
  (params (PlayerIndex :type Integer))
  (return (>= (.y (Transformation|GetActorLocation (Game|GetPlayerCharacter PlayerIndex))) (- (.y (Transformation|GetWorldLocation (Variables|Default|GetSpline))) 1e+02))))

(fn BoxMovement
  (params (PlayerIndex :type Integer))
  (bind _returnvalue (Game|GetPlayerCharacter PlayerIndex))
  (bind _returnvalue_2 (Game|GetPlayerCharacter 0))
  (bind _returnvalue_3 (Utilities|Time|GetWorldDeltaSeconds))
  (bind _speedonzipline (Variables|Default|GetSpeedOnZipline))
  (bind _boxp1 (Variables|Default|GetBoxP1))
  (bind _spline (Variables|Default|GetSpline))
  (bind _spline_2 (Variables|Default|GetSpline))
  (bind _returnvalue_4 (Transformation|GetActorLocation _returnvalue))
  (bind _asbp_punisher (Utilities|Casting|CastToBP_Punisher _returnvalue))
  (bind (_asbp_punisher_2 _bsuccess) (Utilities|Casting|CastToBP_Punisher _returnvalue_2))
  (bind _returnvalue_5 (* _returnvalue_3 _speedonzipline))
  (bind _returnvalue_6 (Utilities|Select :Index PlayerIndex :Option%200 _boxp1 :Option%201 0))
  (bind _returnvalue_7 (Transformation|GetWorldLocation _returnvalue_6))
  (bind _attach (Variables|/Game/Personnage/PunisherNelson/Bp/BP_Punisher.BP_Punisher_C|GetAttach _asbp_punisher))
  (bind _returnvalue_8 (+ (.y _returnvalue_7) _returnvalue_5))
  (bind _returnvalue_9 (select _attach _returnvalue_8 (.y _returnvalue_4)))
  (bind _returnvalue_10 (Spline|FindLocationClosesttoWorldLocation _spline_2 (Math|Vector|MakeVector (.x _returnvalue_7) _returnvalue_9 (.z _returnvalue_7)) "World"))
  (Transformation|SetWorldLocation (Utilities|Select :Index PlayerIndex :Option%200 (Variables|Default|GetBoxP1) :Option%201 (Variables|Default|GetBoxP1)) _returnvalue_10 false false)
  (if (Math|Float|NearlyEqual(Float) (Class|SplineComponent|GetDistanceAlongSplineatLocation _spline _returnvalue_10 "World") (Spline|GetSplineLength _spline) 5e+01)
    (Utilities|FlowControl|Sequence
      (:then_0
        (if (Variables|/Game/Personnage/PunisherNelson/Bp/BP_Punisher.BP_Punisher_C|GetAttach _asbp_punisher_2)
          (Default|ManageZipline _asbp_punisher_2 false)
          (Variables|/Game/Personnage/PunisherNelson/Bp/BP_Punisher.BP_Punisher_C|SetCanAttach _asbp_punisher_2 _bsuccess)))
      (:then_1
        (Components|DestroyComponent (Utilities|Select :Index 0 :Option%200 (Variables|Default|GetBoxP1) :Option%201 (Variables|Default|GetBoxP1)))))))