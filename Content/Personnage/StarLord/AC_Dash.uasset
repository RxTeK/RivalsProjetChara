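; Actor component that gives Star-Lord a dash on right click.
; It launches him upward, then adds a velocity-change impulse along the last movement input, or the spring arm's forward when there is no input, scaled by DashRange.
; A DoOnce gate enforces the cooldown: timers clear the Dash flag shortly after, then re-arm the dash about a second after use.
; Leftover debug prints and a line trace are disconnected.
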(event Custom|DelayDash
  ;[1 0 0.3451] Dash
  (Variables|Default|SetDash! false))

(event Custom|CanDash
  (bind _dashrange (Variables|Default|GetDashRange))
  (bind _starlordref (Variables|Default|GetStarlordREF))
  (bind _starlordref_2 (Variables|Default|GetStarlordREF))
  (bind _charactermovement (Variables|/Script/Engine.Character|GetCharacterMovement _starlordref))
  (bind _springarm (Variables|/Game/Personnage/StarLord/BP_StarLord.BP_StarLord_C|GetSpringArm _starlordref_2))
  (bind _returnvalue (Pawn|Components|PawnMovement|GetLastInputVector _charactermovement))
  (bind _returnvalue_2 (Math|Vector|GetForwardVector _springarm))
  (bind _returnvalue_3 (Utilities|Operators|EqualEqual :A _returnvalue))
  (bind _returnvalue_4 (Math|Vector|SelectVector _returnvalue_2 _returnvalue _returnvalue_3))
  (bind _returnvalue_5 (* _returnvalue_4 _dashrange))
  ;[1 0 0.3451] Dash
  (Utilities|FlowControl|DoOnce false) ; enters at Reset
)

(event Custom|Reset
  ;[1 0 0.3451] Dash
  (CallFunction|CanDash))

(event Input|EnhancedActionEvents|EnhancedInputActionIA_StarLordRightClick
  (params (ActionValue :type Boolean) (ElapsedSeconds :type Float%20%28double-precision%29) (TriggeredSeconds :type Float%20%28double-precision%29) (InputAction :type Input%20Action%20Object%20Reference :default "/Game/Personnage/StarLord/Inputs/IA_StarLordRightClick.IA_StarLordRightClick"))
  (bind _dashrange (Variables|Default|GetDashRange))
  (bind _starlordref (Variables|Default|GetStarlordREF))
  (bind _starlordref_2 (Variables|Default|GetStarlordREF))
  (bind _charactermovement (Variables|/Script/Engine.Character|GetCharacterMovement _starlordref))
  (bind _springarm (Variables|/Game/Personnage/StarLord/BP_StarLord.BP_StarLord_C|GetSpringArm _starlordref_2))
  (bind _returnvalue (Pawn|Components|PawnMovement|GetLastInputVector _charactermovement))
  (bind _returnvalue_2 (Math|Vector|GetForwardVector _springarm))
  (bind _returnvalue_3 (Utilities|Operators|EqualEqual :A _returnvalue))
  (bind _returnvalue_4 (Math|Vector|SelectVector _returnvalue_2 _returnvalue _returnvalue_3))
  (bind _returnvalue_5 (* _returnvalue_4 _dashrange))
  ;[1 0 0.3451] Dash
  (:Started
    (Utilities|FlowControl|DoOnce false
      (:Completed
        (Variables|Default|SetDash! true)
        (Physics|AddImpulse (Variables|/Script/Engine.Character|GetCharacterMovement (Variables|Default|GetStarlordREF)) (Math|Vector|MakeVector 0.0 0.0 5e+02) true)
        (Physics|AddImpulse (Variables|/Script/Engine.Character|GetCharacterMovement (Variables|Default|GetStarlordREF)) (Math|Vector|MakeVector (.x _returnvalue_5) (.y _returnvalue_5) (.z _returnvalue_5)) true)
        (Utilities|Time|SetTimerbyEvent (delegate Custom|DelayDash) 0.7)
        (Utilities|Time|SetTimerbyEvent (delegate Custom|Reset) 1.0)))))

(event EventBeginPlay
  ;[1 0 0.3451] Dash
  (bind _asbp_star_lord (Utilities|Casting|CastToBP_StarLord (Components|GetOwner)))
  (Variables|Default|SetStarlordREF _asbp_star_lord))