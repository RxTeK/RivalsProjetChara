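; Actor component for Star-Lord's primary fire and reload on BP_Player, disabled while AC_AimBot's Aimbot is active.
; Holding input loops a timer that spends ammo, shakes the camera and sphere-traces from the camera with stepped spread, damaging enemy dummies.
; A nonzero AC_Ultimate Hit overrides the trace target.
; An empty magazine or reload input plays a DoOnce-guarded montage, then refills ammo and resumes held fire.
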(event Custom|ShootTime
  (bind _shootnumber (Variables|Default|GetShootNumber))
  (bind _playerref (Variables|Default|GetPlayerREF))
  (bind _playerref_2 (Variables|Default|GetPlayerREF))
  (bind _returnvalue (Actor|GetComponentbyClass _playerref_2 "/Game/Personnage/StarLord/AC_Ultimate.AC_Ultimate_C"))
  (bind _followcamera (Variables|/Game/Personnage/ALL/BP_Player.BP_Player_C|GetFollowCamera _playerref))
  (bind _returnvalue_2 (Transformation|GetWorldLocation _followcamera))
  (bind _hit (Variables|/Game/Personnage/StarLord/AC_Ultimate.AC_Ultimate_C|GetHit _returnvalue))
  ;[0.9906 0.8607 0.08009] Shoot
  (if (and (Variables|Default|GetAction%20Value) (not (Variables|/Game/Personnage/StarLord/AC_AimBot.AC_AimBot_C|GetAimbot! (Actor|GetComponentbyClass (Variables|Default|GetPlayerREF) "/Game/Personnage/StarLord/AC_AimBot.AC_AimBot_C"))))
    (if (not (Variables|Default|GetReload?))
      (Utilities|FlowControl|Sequence
        (:then_0
          (Math|Integer|IncrementInt _shootnumber
            (:%20%20
              (if (> _shootnumber 2)
                (Variables|Default|SetSpread 1e+07)
                (if (> _shootnumber 5)
                  (Variables|Default|SetSpread 2e+07))))))
        (:then_1
          (Variables|Default|SetShoot! true)
          (Variables|Default|SetAmmo (- (Variables|Default|GetAmmo) 2))
          (Camera|PlayWorldCameraShake "/Game/Personnage/StarLord/CS_ShootShake.CS_ShootShake_C" (Transformation|GetActorLocation (Variables|Default|GetPlayerREF)) 5e+02 2e+03)
          (if (== (Variables|Default|GetAmmo) 0)
            (CallFunction|Reload)
            (else
              (bind _outhit (Collision|SphereTraceByChannel _returnvalue_2 (Math|Vector|SelectVector (+ _returnvalue_2 (* (Math|Vector|GetForwardVector _followcamera) 1000000000) (Math|Vector|MakeVector (Math|Random|RandomFloatinRange (* (Variables|Default|GetSpread) -1.0) (Variables|Default|GetSpread)) (Math|Random|RandomFloatinRange (* (Variables|Default|GetSpread) -1.0) (Variables|Default|GetSpread)) (Math|Random|RandomFloatinRange (* (Variables|Default|GetSpread) -1.0) (Variables|Default|GetSpread)))) _hit (Utilities|Operators|EqualEqual :A _hit)) 5.0 "TraceTypeQuery3" false 0 "ForDuration" true "(R=1.000000,G=0.000000,B=0.000000,A=1.000000)" "(R=0.000000,G=1.000000,B=0.000000,A=1.000000)" 0.5))
              (Utilities|IsValid (.AsBP%20Dummy (Utilities|Casting|CastToBP_Dummy (.HitActor (Collision|BreakHitResult _outhit))))
                (:Is%20Valid
                  (if (Utilities|Select :Index (Variables|/Game/Personnage/Dummy/BP_Dummy.BP_Dummy_C|GetDummyType (.AsBP%20Dummy (Utilities|Casting|CastToBP_Dummy (.HitActor (Collision|BreakHitResult _outhit))))) :NewEnumerator0 true :NewEnumerator1 false)
                    (Game|Damage|ApplyDamage (.AsBP%20Dummy (Utilities|Casting|CastToBP_Dummy (.HitActor (Collision|BreakHitResult _outhit)))) (Variables|Default|GetDamage) 0 0)))))))))))

(event Custom|Reload
  ;[0.9906 0.8607 0.08009] Shoot
  ;;[0.07762 0.899 0.1147] Reload
  (Utilities|FlowControl|DoOnce false
    (:Completed
      (Variables|Default|SetReload? true)
      (Development|PrintString "Hello")
      (Animation|Montage|PlayMontage (Variables|/Script/Engine.Character|GetMesh (Variables|Default|GetPlayerREF)) "/Game/Personnage/StarLord/TEST_EXPORT/AnimRetargeted/AM_StarlordReloadGround.AM_StarlordReloadGround"
        (:OnCompleted
          (CallFunction|ReloadReset)
          (Variables|Default|SetFirstShoot? true)
          (Variables|Default|SetShootNumber 0)
          (Variables|Default|SetSpread 0.0)
          (Variables|Default|SetAmmo 40)
          (Variables|Default|SetReload? false)
          (CallFunction|ShootAuto))))))

(event Custom|ShootAuto
  ;[0.9906 0.8607 0.08009] Shoot
  (if (not (Variables|Default|GetReload?))
    (Utilities|FlowControl|Sequence
      (:then_0
        (if (Variables|Default|GetAction%20Value)
          (if (Variables|Default|GetFirstShoot?)
            (Variables|Default|SetFirstShoot? false)
            (CallFunction|ShootTime))))
      (:then_1
        (if (== (Variables|Default|GetAmmo) 0)
          (CallFunction|Reload)
          (else
            (bind _returnvalue (Utilities|Time|SetTimerbyEvent (delegate Custom|ShootTime) 0.05 true))
            (Variables|Default|SetShootHandleTimer _returnvalue)))))))

(event Custom|ReloadReset
  ;[0.9906 0.8607 0.08009] Shoot
  ;;[0.07762 0.899 0.1147] Reload
  (Utilities|FlowControl|DoOnce false) ; enters at Reset
)

(event Input|EnhancedActionEvents|EnhancedInputActionIA_StarLordNormal
  (params (ActionValue :type Boolean) (ElapsedSeconds :type Float%20%28double-precision%29) (TriggeredSeconds :type Float%20%28double-precision%29) (InputAction :type Input%20Action%20Object%20Reference :default "/Game/Personnage/StarLord/Inputs/IA_StarLordNormal.IA_StarLordNormal"))
  ;[0.9906 0.8607 0.08009] Shoot
  (:Triggered
    (Variables|Default|SetAction%20Value ActionValue))
  (:Started
    (if (not (Variables|/Game/Personnage/StarLord/AC_AimBot.AC_AimBot_C|GetAimbot! (Actor|GetComponentbyClass (Variables|Default|GetPlayerREF) "/Game/Personnage/StarLord/AC_AimBot.AC_AimBot_C")))
      (Variables|Default|SetShoot! false)
      (if (not (Variables|Default|GetReload?))
        (Utilities|FlowControl|Sequence
          (:then_0
            (if (Variables|Default|GetAction%20Value)
              (if (Variables|Default|GetFirstShoot?)
                (Variables|Default|SetFirstShoot? false)
                (CallFunction|ShootTime))))
          (:then_1
            (if (== (Variables|Default|GetAmmo) 0)
              (CallFunction|Reload)
              (else
                (bind _returnvalue (Utilities|Time|SetTimerbyEvent (delegate Custom|ShootTime) 0.05 true))
                (Variables|Default|SetShootHandleTimer _returnvalue))))))))
  (:Completed
    (Variables|Default|SetAction%20Value false)
    (Utilities|Time|ClearandInvalidateTimerbyHandle (Variables|Default|GetShootHandleTimer))
    (if (Variables|Default|GetReload?)
      _
      (else
        (Utilities|Time|ClearandInvalidateTimerbyHandle (Variables|Default|GetShootHandleTimer))))
    (Variables|Default|SetFirstShoot? true)
    (Variables|Default|SetShootNumber 0)
    (Variables|Default|SetSpread 0.0)))

(event Input|EnhancedActionEvents|EnhancedInputActionIA_StarLordReload
  (params (ActionValue :type Boolean) (ElapsedSeconds :type Float%20%28double-precision%29) (TriggeredSeconds :type Float%20%28double-precision%29) (InputAction :type Input%20Action%20Object%20Reference :default "/Game/Personnage/StarLord/Inputs/IA_StarLordReload.IA_StarLordReload"))
  ;[0.9906 0.8607 0.08009] Shoot
  ;;[0.07762 0.899 0.1147] Reload
  (:Started
    (if (< (Variables|Default|GetAmmo) (Variables|Default|GetAmmoMax))
      (Utilities|FlowControl|DoOnce false
        (:Completed
          (Variables|Default|SetReload? true)
          (Development|PrintString "Hello")
          (Animation|Montage|PlayMontage (Variables|/Script/Engine.Character|GetMesh (Variables|Default|GetPlayerREF)) "/Game/Personnage/StarLord/TEST_EXPORT/AnimRetargeted/AM_StarlordReloadGround.AM_StarlordReloadGround"
            (:OnCompleted
              (CallFunction|ReloadReset)
              (Variables|Default|SetFirstShoot? true)
              (Variables|Default|SetShootNumber 0)
              (Variables|Default|SetSpread 0.0)
              (Variables|Default|SetAmmo 40)
              (Variables|Default|SetReload? false)
              (CallFunction|ShootAuto))))))))

(event EventBeginPlay
  ;[0.9906 0.8607 0.08009] Shoot
  (bind _asbp_player (Utilities|Casting|CastToBP_Player (Components|GetOwner)))
  (Variables|Default|SetPlayerREF _asbp_player))