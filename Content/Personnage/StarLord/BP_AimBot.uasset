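; StarLord's E skill, an aimbot-style auto-damage ability owned by BP_StarLord and triggered by IA_StarlordE.
; While active, a looping timer repeatedly sphere-traces around StarLord, with debug drawing, and damages BP_Dummy hits of one DummyType.
; ActorsToIgnore de-duplicates each pulse's hits and is cleared afterwards.
; After three seconds it clears the Aimbot flag and starts a cooldown timer that resets the DoOnce gate.
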(event Custom|E_SkillLoop
  (bind _starlordref (Variables|Default|GetStarLordREF))
  (bind _actors_to_ignore (Variables|Default|GetActors%20to%20Ignore))
  (bind _returnvalue (Transformation|GetActorLocation _starlordref))
  (Variables|Default|SetTime (+ (Variables|Default|GetTime) 0.1))
  (if (>= (Variables|Default|GetTime) 3.0)
    (Utilities|Time|ClearandInvalidateTimerbyHandle (Variables|Default|GetE_SkillHandle))
    (Variables|Default|SetTime 0.0)
    (Variables|Default|SetAimbot! false)
    (Development|PrintString "Hello")
    (Utilities|Time|SetTimerbyEvent (delegate Custom|Reset_E) 8.0)
    (else
      (bind _outhits (Collision|MultiSphereTraceByChannel _returnvalue _returnvalue 8e+02 "TraceTypeQuery3" false (Variables|Default|GetActors%20to%20Ignore) "ForDuration" true "(R=1.000000,G=0.000000,B=0.000000,A=1.000000)" "(R=0.000000,G=1.000000,B=0.000000,A=1.000000)" 0.5))
      (for _array_element _outhits
        (if (== (Utilities|Array|FindItem (Variables|Default|GetActors%20to%20Ignore) (.AsBP%20Dummy (Utilities|Casting|CastToBP_Dummy (.HitActor (Collision|BreakHitResult _array_element))))) -1)
          (Utilities|Array|Add (Variables|Default|GetActors%20to%20Ignore) (.AsBP%20Dummy (Utilities|Casting|CastToBP_Dummy (.HitActor (Collision|BreakHitResult _array_element)))))
          (Development|PrintString (Utilities|GetDisplayName (.AsBP%20Dummy (Utilities|Casting|CastToBP_Dummy (.HitActor (Collision|BreakHitResult _array_element))))) true true "(R=1.000000,G=0.938499,B=0.000000,A=1.000000)")))
      (for _array_element_2 _actors_to_ignore
        (if (Utilities|Enum|Equal(Enum) (Variables|/Game/Personnage/Dummy/BP_Dummy.BP_Dummy_C|GetDummyType _array_element_2) "NewEnumerator0")
          (Game|Damage|ApplyDamage _array_element_2 8.0 0 0)))
      (Utilities|Array|Clear _actors_to_ignore))))

(event Custom|Reset_E
  (Utilities|FlowControl|DoOnce false) ; enters at Reset
)

(event Input|EnhancedActionEvents|EnhancedInputActionIA_StarlordE
  (params (ActionValue :type Boolean) (ElapsedSeconds :type Float%20%28double-precision%29) (TriggeredSeconds :type Float%20%28double-precision%29) (InputAction :type Input%20Action%20Object%20Reference :default "/Game/Personnage/StarLord/Inputs/IA_StarlordE.IA_StarlordE"))
  (:Started
    (Utilities|FlowControl|DoOnce false
      (:Completed
        (Variables|Default|SetAimbot! true)
        (bind _returnvalue (Utilities|Time|SetTimerbyEvent (delegate Custom|E_SkillLoop) 0.1 true))
        (Variables|Default|SetE_SkillHandle _returnvalue)))))

(event EventBeginPlay
  (bind _asbp_star_lord (Utilities|Casting|CastToBP_StarLord (Components|GetOwner)))
  (Variables|Default|SetStarLordREF _asbp_star_lord))