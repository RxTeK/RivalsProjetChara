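; Component on BP_StarLord that handles the character's automatic primary fire and reload, disabled while the aimbot is active.
; A looping timer fires sphere traces from the camera toward the aim-assist point, or forward with spread that grows over consecutive shots, damaging BP_Dummy actors.
; An empty magazine or reload input starts a timed reload that resumes fire if held.
; Debug trace drawing and per-tick aim-assist printing remain enabled.
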(event Custom|ShootTime
  (bind _starlordref (Variables|Default|GetStarlordREF))
  (bind _starlordref_2 (Variables|Default|GetStarlordREF))
  (bind _shootnumber (Variables|Default|GetShootNumber))
  (bind _camera (Variables|/Game/Personnage/StarLord/BP_StarLord.BP_StarLord_C|GetCamera _starlordref_2))
  (bind _bp_aimassist (Variables|/Game/Personnage/StarLord/BP_StarLord.BP_StarLord_C|GetBP_AimAssist _starlordref))
  (bind _returnvalue (Transformation|GetWorldLocation _camera))
  (bind _hit (Variables|/Game/Personnage/StarLord/BP_Ultimate.BP_Ultimate_C|GetHit _bp_aimassist))
  ;[0.9906 0.8607 0.08009] Shoot
  (if (and (Variables|Default|GetAction%20Value) (not (Variables|/Game/Personnage/StarLord/BP_AimBot.BP_AimBot_C|GetAimbot! (Variables|/Game/Personnage/StarLord/BP_StarLord.BP_StarLord_C|GetBP_AimBot (Variables|Default|GetStarlordREF)))))
    (if (not (Variables|Default|GetReload?))
      (Utilities|FlowControl|Sequence
        (:then_0
          (Math|Integer|IncrementInt _shootnumber
            (:%20%20
              (if (> _shootnumber 2)
                (Variables|Default|SetSpread 1e+07)
                (if (> _shootnumber 5)
                  (Variables|Default|SetSpread 2e+07))))))
        (:then_1
          (Variables|Default|SetShoot! true)
          (Variables|Default|SetAmmo (- (Variables|Default|GetAmmo) 2))
          (if (== (Variables|Default|GetAmmo) 0)
            (CallFunction|Reload)
            (else
              (bind _outhit (Collision|SphereTraceByChannel _returnvalue (Math|Vector|SelectVector (+ _returnvalue (* (Math|Vector|GetForwardVector _camera) 1000000000) (Math|Vector|MakeVector (Math|Random|RandomFloatinRange (* (Variables|Default|GetSpread) -1.0) (Variables|Default|GetSpread)) (Math|Random|RandomFloatinRange (* (Variables|Default|GetSpread) -1.0) (Variables|Default|GetSpread)) (Math|Random|RandomFloatinRange (* (Variables|Default|GetSpread) -1.0) (Variables|Default|GetSpread)))) _hit (Utilities|Operators|EqualEqual :A _hit)) 5.0 "TraceTypeQuery3" false 0 "ForDuration" true "(R=1.000000,G=0.000000,B=0.000000,A=1.000000)" "(R=0.000000,G=1.000000,B=0.000000,A=1.000000)" 0.5))
              (Game|Damage|ApplyDamage (.AsBP%20Dummy (Utilities|Casting|CastToBP_Dummy (.HitActor (Collision|BreakHitResult _outhit)))) (Variables|Default|GetDamage) 0 0))))))))

(event Custom|ReloadTime
  ;[0.9906 0.8607 0.08009] Shoot
  ;;[0.07762 0.899 0.1147] Reload
  (Variables|Default|SetFirstShoot? true)
  (Variables|Default|SetShootNumber 0)
  (Variables|Default|SetSpread 0.0)
  (Variables|Default|SetAmmo 40)
  (Variables|Default|SetReload? false)
  (CallFunction|ShootAuto))

(event Custom|Reload
  ;[0.9906 0.8607 0.08009] Shoot
  ;;[0.07762 0.899 0.1147] Reload
  (Variables|Default|SetReload? true)
  (Utilities|Time|SetTimerbyEvent (delegate Custom|ReloadTime) 0.6))

(event Custom|ShootAuto
  ;[0.9906 0.8607 0.08009] Shoot
  (if (not (Variables|Default|GetReload?))
    (Utilities|FlowControl|Sequence
      (:then_0
        (if (Variables|Default|GetAction%20Value)
          (if (Variables|Default|GetFirstShoot?)
            (Variables|Default|SetFirstShoot? false)
            (CallFunction|ShootTime))))
      (:then_1
        (if (== (Variables|Default|GetAmmo) 0)
          (CallFunction|Reload)
          (else
            (bind _returnvalue (Utilities|Time|SetTimerbyEvent (delegate Custom|ShootTime) 0.05 true))
            (Variables|Default|SetShootHandleTimer _returnvalue)))))))

(event Input|EnhancedActionEvents|EnhancedInputActionIA_StarLordNormal
  (params (ActionValue :type Boolean) (ElapsedSeconds :type Float%20%28double-precision%29) (TriggeredSeconds :type Float%20%28double-precision%29) (InputAction :type Input%20Action%20Object%20Reference :default "/Game/Personnage/StarLord/Inputs/IA_StarLordNormal.IA_StarLordNormal"))
  ;[0.9906 0.8607 0.08009] Shoot
  (:Triggered
    (Variables|Default|SetAction%20Value ActionValue))
  (:Started
    (if (not (Variables|/Game/Personnage/StarLord/BP_AimBot.BP_AimBot_C|GetAimbot! (Variables|/Game/Personnage/StarLord/BP_StarLord.BP_StarLord_C|GetBP_AimBot (Variables|Default|GetStarlordREF))))
      (Variables|Default|SetShoot! false)
      (if (not (Variables|Default|GetReload?))
        (Utilities|FlowControl|Sequence
          (:then_0
            (if (Variables|Default|GetAction%20Value)
              (if (Variables|Default|GetFirstShoot?)
                (Variables|Default|SetFirstShoot? false)
                (CallFunction|ShootTime))))
          (:then_1
            (if (== (Variables|Default|GetAmmo) 0)
              (CallFunction|Reload)
              (else
                (bind _returnvalue (Utilities|Time|SetTimerbyEvent (delegate Custom|ShootTime) 0.05 true))
                (Variables|Default|SetShootHandleTimer _returnvalue))))))))
  (:Completed
    (Variables|Default|SetAction%20Value false)
    (Utilities|Time|ClearandInvalidateTimerbyHandle (Variables|Default|GetShootHandleTimer))
    (if (Variables|Default|GetReload?)
      _
      (else
        (Utilities|Time|ClearandInvalidateTimerbyHandle (Variables|Default|GetShootHandleTimer))))
    (Variables|Default|SetFirstShoot? true)
    (Variables|Default|SetShootNumber 0)
    (Variables|Default|SetSpread 0.0)))

(event Input|EnhancedActionEvents|EnhancedInputActionIA_StarLordReload
  (params (ActionValue :type Boolean) (ElapsedSeconds :type Float%20%28double-precision%29) (TriggeredSeconds :type Float%20%28double-precision%29) (InputAction :type Input%20Action%20Object%20Reference :default "/Game/Personnage/StarLord/Inputs/IA_StarLordReload.IA_StarLordReload"))
  ;[0.9906 0.8607 0.08009] Shoot
  ;;[0.07762 0.899 0.1147] Reload
  (:Started
    (if (< (Variables|Default|GetAmmo) (Variables|Default|GetAmmoMax))
      (Variables|Default|SetReload? true)
      (Utilities|Time|SetTimerbyEvent (delegate Custom|ReloadTime) 0.6))))

(event EventTick
  (params (DeltaSeconds :type Float%20%28single-precision%29))
  (Development|PrintString (Utilities|String|ToString(Vector) (Variables|/Game/Personnage/StarLord/BP_Ultimate.BP_Ultimate_C|GetHit (Variables|/Game/Personnage/StarLord/BP_StarLord.BP_StarLord_C|GetBP_AimAssist (Variables|Default|GetStarlordREF)))) true true "(R=1.000000,G=0.822387,B=0.000000,A=1.000000)" 0.0))

(event EventBeginPlay
  (bind _asbp_star_lord (Utilities|Casting|CastToBP_StarLord (Components|GetOwner)))
  (Variables|Default|SetStarlordREF _asbp_star_lord))