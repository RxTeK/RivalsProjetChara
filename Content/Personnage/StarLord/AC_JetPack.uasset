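; Star-Lord jetpack component that toggles the player between walking and flying on Shift, gated by fuel and blocked during Ultimate.
; While active, a looping timer burns fuel and pushes the player along control yaw, with separate up/down input.
; Shutdown by toggle or empty tank relaunches the player at half the last velocity.
; Only running empty starts timed fuel regeneration; activating Ultimate cuts thrust without resetting movement mode.
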(event Custom|JetPackSpeed
  ;[1 0.4217 0] JetPack
  (Variables|Default|SetFuel (Math|Integer|Clamp(Integer) (- (Variables|Default|GetFuel) 3) 0 (Variables|Default|GetFuelMax)))
  (if (== (Variables|Default|GetFuel) 0)
    (CallFunction|FuelReload)
    (Pawn|Components|CharacterMovement|SetMovementMode (Variables|/Script/Engine.Character|GetCharacterMovement (Variables|Default|GetPlayerREF)) "MOVE_Walking" 0)
    (Audio|Components|Audio|Stop (Variables|Default|GetSoundREF))
    (Audio|PlaySoundatLocation "/Game/Personnage/StarLord/Sound/FX_StarlordJetpackEnd.FX_StarlordJetpackEnd" (Transformation|GetActorLocation (Variables|Default|GetPlayerREF)) "0, 0, 0" 1.0 1.0 0.0 0 0 0 0)
    (Utilities|Time|ClearandInvalidateTimerbyHandle (Variables|Default|GetJetPackSpeedHandle))
    (Character|LaunchCharacter (Variables|Default|GetPlayerREF) (/ (Variables|Default|GetLastVelocity) 2) false true)
    (elif (Variables|/Game/Personnage/StarLord/AC_Ultimate.AC_Ultimate_C|GetUltimate! (Actor|GetComponentbyClass (Variables|Default|GetPlayerREF) "/Game/Personnage/StarLord/AC_Ultimate.AC_Ultimate_C"))
      (Audio|Components|Audio|Stop (Variables|Default|GetSoundREF))
      (Audio|PlaySoundatLocation "/Game/Personnage/StarLord/Sound/FX_StarlordJetpackEnd.FX_StarlordJetpackEnd" (Transformation|GetActorLocation (Variables|Default|GetPlayerREF)) "0, 0, 0" 1.0 1.0 0.0 0 0 0 0)
      (Utilities|Time|ClearandInvalidateTimerbyHandle (Variables|Default|GetJetPackSpeedHandle))
      (Variables|Default|SetJetPack! false)
      (else
        (Pawn|Input|AddMovementInput (Variables|Default|GetPlayerREF) (Math|Vector|GetForwardVector (Math|Rotator|MakeRotator 0.0 0.0 (.yaw (Pawn|GetControlRotation (Variables|Default|GetPlayerREF) :!class /Script/Engine.Pawn)))) 1.0 false)
        (Variables|Default|SetLastVelocity (Transformation|GetVelocity (Variables|Default|GetPlayerREF)))))))

(event Custom|RegenFuel
  ;[1 0.4217 0] JetPack
  (Variables|Default|SetFuel (Math|Integer|Clamp(Integer) (+ (Variables|Default|GetFuel) 1) 0 (Variables|Default|GetFuelMax)))
  (if (== (Variables|Default|GetFuel) (Variables|Default|GetFuelMax))
    (Utilities|Time|ClearandInvalidateTimerbyHandle (Variables|Default|GetRegenFuelHandle))))

(event Custom|FuelReload
  ;[1 0.4217 0] JetPack
  (Variables|Default|SetJetPack! false)
  (bind _returnvalue (Utilities|Time|SetTimerbyEvent (delegate Custom|RegenFuel) 0.01 true))
  (Variables|Default|SetRegenFuelHandle _returnvalue))

(event Input|EnhancedActionEvents|EnhancedInputActionIA_StarLordShift
  (params (ActionValue :type Boolean) (ElapsedSeconds :type Float%20%28double-precision%29) (TriggeredSeconds :type Float%20%28double-precision%29) (InputAction :type Input%20Action%20Object%20Reference :default "/Game/Personnage/StarLord/Inputs/IA_StarLordShift.IA_StarLordShift"))
  ;[1 0.4217 0] JetPack
  (:Started
    (if (not (Variables|/Game/Personnage/StarLord/AC_Ultimate.AC_Ultimate_C|GetUltimate! (Actor|GetComponentbyClass (Variables|Default|GetPlayerREF) "/Game/Personnage/StarLord/AC_Ultimate.AC_Ultimate_C")))
      (if (> (Variables|Default|GetFuel) 300)
        (if (Variables|Default|GetJetPack!)
          (Variables|Default|SetJetPack! false)
          (Pawn|Components|CharacterMovement|SetMovementMode (Variables|/Script/Engine.Character|GetCharacterMovement (Variables|Default|GetPlayerREF)) "MOVE_Walking" 0)
          (Audio|Components|Audio|Stop (Variables|Default|GetSoundREF))
          (Audio|PlaySoundatLocation "/Game/Personnage/StarLord/Sound/FX_StarlordJetpackEnd.FX_StarlordJetpackEnd" (Transformation|GetActorLocation (Variables|Default|GetPlayerREF)) "0, 0, 0" 1.0 1.0 0.0 0 0 0 0)
          (Utilities|Time|ClearandInvalidateTimerbyHandle (Variables|Default|GetJetPackSpeedHandle))
          (Character|LaunchCharacter (Variables|Default|GetPlayerREF) (/ (Variables|Default|GetLastVelocity) 2) false true)
          (else
            (Audio|PlaySound2D "/Game/Personnage/StarLord/Sound/FX_StarlordJetpackStart.FX_StarlordJetpackStart" 1.0 1.0 0.0 0 0)
            (bind _returnvalue (Audio|SpawnSound2D "/Game/Personnage/StarLord/Sound/FX_StarlordJetpackLoop.FX_StarlordJetpackLoop" 1.0 1.0 0.0 0))
            (Variables|Default|SetSoundREF _returnvalue)
            (Camera|PlayWorldCameraShake "/Game/Personnage/StarLord/CameraShake/CS_Jetpack.CS_Jetpack_C" (Transformation|GetActorLocation (Variables|Default|GetPlayerREF)) 1e+03 1e+03)
            (Variables|Default|SetJetPack! true)
            (Pawn|Components|CharacterMovement|SetMovementMode (Variables|/Script/Engine.Character|GetCharacterMovement (Variables|Default|GetPlayerREF)) "MOVE_Flying" 0)
            (Utilities|Time|ClearandInvalidateTimerbyHandle (Variables|Default|GetRegenFuelHandle))
            (bind _returnvalue_2 (Utilities|Time|SetTimerbyEvent (delegate Custom|JetPackSpeed) 0.01 true))
            (Variables|Default|SetJetPackSpeedHandle _returnvalue_2)))))))

(event Input|EnhancedActionEvents|EnhancedInputActionIA_StarLordFlyUpAndDown
  (params (ActionValue :type Vector%202D%20Structure) (ElapsedSeconds :type Float%20%28double-precision%29) (TriggeredSeconds :type Float%20%28double-precision%29) (InputAction :type Input%20Action%20Object%20Reference :default "/Game/Personnage/StarLord/Inputs/IA_StarLordFlyUpAndDown.IA_StarLordFlyUpAndDown"))
  ;[1 0.4217 0] JetPack
  (:Triggered
    (bind _output_get (Variables|Default|SetUpAndDownValue (.x ActionValue)))
    (if (Class|NavMovementComponent|IsFlying (Variables|/Script/Engine.Character|GetCharacterMovement (Variables|Default|GetPlayerREF)))
      (Pawn|Input|AddMovementInput (Variables|Default|GetPlayerREF) (Transformation|GetActorUpVector (Pawn|GetController (Variables|Default|GetPlayerREF))) _output_get false)))
  (:Completed
    (Variables|Default|SetUpAndDownValue 0.0)))

(event EventBeginPlay
  ;[1 0.4217 0] JetPack
  (bind _asbp_player (Utilities|Casting|CastToBP_Player (Components|GetOwner)))
  (Variables|Default|SetPlayerREF _asbp_player))