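; Star-Lord's ultimate ability component on BP_Player: at full energy it launches the player into flight with an auto-aim crosshair.
; Input plays the montage with controls disabled, then adds the aim widget.
; A looping timer sphere-traces from screen center, picks the enemy dummy nearest center, stores its pelvis as Hit and moves the crosshair there.
; After ten one-second ticks, it restores walking, removes the widget, empties energy and re-arms.
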(event Custom|DelayUltime
  (bind _delayultimate (Variables|Default|GetDelayUltimate))
  ;[0.6618 0 1] Ultimate
  (Math|Float|IncrementFloat _delayultimate
    (:%20%20
      (if (== _delayultimate 1e+01)
        (Utilities|Time|ClearandInvalidateTimerbyHandle (Variables|Default|GetUltimateHandle))
        (Variables|Default|SetUltimate! false)
        (Widget|RemovefromParent (Variables|Default|GetAimREF))
        (Pawn|Components|CharacterMovement|SetMovementMode (Variables|/Script/Engine.Character|GetCharacterMovement (Variables|Default|GetPlayerREF)) "MOVE_Walking" 0)
        (Utilities|Time|ClearandInvalidateTimerbyHandle (Variables|Default|GetAutoAimHandle))
        (Variables|Default|SetHit "0, 0, 0")
        (Variables|/Game/Personnage/ALL/BP_Player.BP_Player_C|SetEnergy (Variables|Default|GetPlayerREF) 0.0)
        (CallFunction|ResetUlti)))))

(event Custom|ExecuteSystem
  ;[0.6618 0 1] Ultimate
  (bind _spawnscreenlocation (CallFunction|SearchforPawntoEngageon))
  (if (Utilities|Operators|NotEqual(!=) :A _spawnscreenlocation)
    (Variables|/Game/Personnage/StarLord/WBP_Aim.WBP_Aim_C|SetCrossHairLocation (Variables|Default|GetAimREF) _spawnscreenlocation)))

(event Custom|ResetUlti
  ;[0.6618 0 1] Ultimate
  (Utilities|FlowControl|DoOnce false) ; enters at Reset
)

(event Input|EnhancedActionEvents|EnhancedInputActionIA_StarLordUlti
  (params (ActionValue :type Boolean) (ElapsedSeconds :type Float%20%28double-precision%29) (TriggeredSeconds :type Float%20%28double-precision%29) (InputAction :type Input%20Action%20Object%20Reference :default "/Game/Personnage/StarLord/Inputs/IA_StarLordUlti.IA_StarLordUlti"))
  (bind _playerref (Variables|Default|GetPlayerREF))
  ;[0.6618 0 1] Ultimate
  (:Started
    (if (== (Variables|/Game/Personnage/ALL/BP_Player.BP_Player_C|GetEnergy _playerref) (Variables|/Game/Personnage/ALL/BP_Player.BP_Player_C|GetMax%20Energy _playerref))
      (Utilities|FlowControl|DoOnce false
        (:Completed
          (Variables|Default|SetUltimate! true)
          (bind _returnvalue (Utilities|Time|SetTimerbyEvent (delegate Custom|ExecuteSystem) 0.016667 true))
          (Variables|Default|SetAutoAimHandle _returnvalue)
          (bind _returnvalue_2 (Utilities|Time|SetTimerbyEvent (delegate Custom|DelayUltime) 1.0 true))
          (Variables|Default|SetUltimateHandle _returnvalue_2)
          (Physics|AddImpulse (Variables|/Script/Engine.Character|GetCharacterMovement (Variables|Default|GetPlayerREF)) "0.000000,0.000000,1000.000000" true)
          (Input|DisableInput (Variables|Default|GetPlayerREF) 0)
          (Animation|Montage|PlayMontage (Variables|/Script/Engine.Character|GetMesh (Variables|Default|GetPlayerREF)) "/Game/Personnage/StarLord/TEST_EXPORT/AnimRetargeted/AnimMontage/AM_UltimateStarlord.AM_UltimateStarlord"
            (:then
              (Pawn|Components|CharacterMovement|SetMovementMode (Variables|/Script/Engine.Character|GetCharacterMovement (Variables|Default|GetPlayerREF)) "MOVE_Flying" 0))
            (:OnCompleted
              (Input|EnableInput (Variables|Default|GetPlayerREF) 0)
              (bind _returnvalue_3 (UserInterface|CreateWidget "/Game/Personnage/StarLord/WBP_Aim.WBP_Aim_C"))
              (bind _output_get (Variables|Default|SetAimREF _returnvalue_3))
              (UserInterface|Viewport|AddtoViewport _output_get 0)
              (Variables|Default|SetUltimate! true))))))))

(event EventBeginPlay
  ;[0.6618 0 1] Ultimate
  (bind _asbp_player (Utilities|Casting|CastToBP_Player (Components|GetOwner)))
  (Variables|Default|SetPlayerREF _asbp_player)
  (Variables|/Game/Personnage/ALL/BP_Player.BP_Player_C|SetEnergy (Variables|Default|GetPlayerREF) 1e+02))

(fn SearchforPawntoEngageon
  (bind _returnvalue (Viewport|GetViewportSize))
  (bind _returnvalue_2 (Game|GetPlayerController 0))
  (bind _l_hittedpawbsdisttocenter (LocalVariables|GetL_HittedPawbsDistToCenter))
  (bind _returnvalue_3 (* _returnvalue 0.5))
  (bind (_worldposition _worlddirection) (Class|GameplayStatics|DeprojectScreentoWorld _returnvalue_2 _returnvalue_3))
  (bind (_outhits _returnvalue_4) (Collision|MultiSphereTraceForObjects (+ _worldposition (* _worlddirection (Variables|Default|GetSearchTraceStartOffset))) (+ _worldposition (* _worlddirection (Variables|Default|GetSearchTraceRange))) (Variables|Default|GetSearchTraceSphereRadius) (Utilities|Array|MakeArray "ObjectTypeQuery3") false (Utilities|Array|MakeArray (Game|Player|GetPlayerPawn 0)) "ForOneFrame"))
  (if _returnvalue_4
    (for _array_element _outhits
      (Utilities|IsValid (.AsBP%20Dummy (Utilities|Casting|CastToBP_Dummy (.HitActor (Collision|BreakHitResult _array_element))))
        (:Is%20Valid
          (if (Utilities|Select :Index (Variables|/Game/Personnage/Dummy/BP_Dummy.BP_Dummy_C|GetDummyType (.AsBP%20Dummy (Utilities|Casting|CastToBP_Dummy (.HitActor (Collision|BreakHitResult _array_element))))) :NewEnumerator0 true :NewEnumerator1 false)
            (Utilities|Map|Add (LocalVariables|GetL_HittedPawbsDistToCenter) (.HitActor (Collision|BreakHitResult _array_element)) (Math|Vector|Distance2D(Vector) (* (Viewport|GetViewportSize) 0.5) (.ScreenPosition (Class|GameplayStatics|ProjectWorldtoScreen (Game|GetPlayerController 0) (Transformation|GetActorLocation (.HitActor (Collision|BreakHitResult _array_element))) false))))))))
    (bind _keys (Utilities|Map|Keys _l_hittedpawbsdisttocenter))
    (bind _values (Utilities|Map|Values _l_hittedpawbsdisttocenter))
    (Utilities|IsValid (Utilities|Array|Get(acopy) _keys (.IndexOfMinValue (Math|Float|MinOfFloatArray _values)))
      (:Is%20Valid
        (bind _ascharacter (Utilities|Casting|CastToCharacter (Utilities|Array|Get(acopy) _keys (.IndexOfMinValue (Math|Float|MinOfFloatArray _values)))))
        (Variables|Default|SetHit (Transformation|GetSocketLocation (Variables|/Script/Engine.Character|GetMesh _ascharacter) "pelvis"))
        (return (.ScreenPosition (Class|WidgetLayoutLibrary|ProjectWorldLocationtoWidgetPosition (Game|GetPlayerController 0) (Transformation|GetSocketLocation (Variables|/Script/Engine.Character|GetMesh _ascharacter) "pelvis") false)))))
    (else
      (Variables|Default|SetHit "0, 0, 0")
      (return "(X=0.000000,Y=0.000000)"))))

(fn AjustCrosshairScreenLocation
  (params (EngagePawnScreenLocation :type Vector%202D%20Structure) (NewParam :type Actor%20Object%20Reference))
  (bind _output_get (LocalVariables|SetL_EngagedPawnScreenLocation (.ScreenPosition (Class|GameplayStatics|ProjectWorldtoScreen (Game|GetPlayerController 0) (Transformation|GetActorLocation NewParam) false))))
  (return _output_get))

(fn GetCrosshairLocation
  (return (Variables|Default|GetCrosshairScreenLocation)))