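; BP_WinterHook is a hook projectile for the WinterSoldier character that pulls a hit target back to where the hook spawned.
; It records its spawn location on BeginPlay and destroys itself on Tick once it travels beyond Range, scaled by 100.
; When its sphere overlaps a Character or Pawn, it moves that actor instantly to the spawn point without sweeping, applies fixed damage, then destroys itself.
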(event OnComponentBeginOverlap(Sphere)
  (params (OverlappedComponent :type Primitive%20Component%20Object%20Reference) (OtherActor :type Actor%20Object%20Reference) (OtherComp :type Primitive%20Component%20Object%20Reference) (OtherBodyIndex :type Integer) (bFromSweep :type Boolean) (SweepResult :type Hit%20Result%20Structure%20%28by%20ref%29))
  (Utilities|Casting|CastToCharacter OtherActor
    (:then
      _)
    (:CastFailed
      (Utilities|Casting|CastToPawn OtherActor)))
  (Transformation|SetActorLocation OtherActor (Variables|Default|GetStart%20location) false false)
  (Game|Damage|ApplyDamage OtherActor 15.0 0 0)
  (Actor|DestroyActor))

(event EventBeginPlay
  (Variables|Default|SetStart%20location (Transformation|GetActorLocation)))

(event EventTick
  (params (DeltaSeconds :type Float%20%28single-precision%29))
  (if (> (Math|Vector|Distance(Vector) (Transformation|GetActorLocation) (Variables|Default|GetStart%20location)) (* (Variables|Default|GetRange) 1e+02))
    (Actor|DestroyActor)))

(fn ConstructionScript)