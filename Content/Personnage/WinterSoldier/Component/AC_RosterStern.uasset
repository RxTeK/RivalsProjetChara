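; Weapon component for the Winter Soldier player character that handles shooting and reloading.
; Attack traces from the camera to find the aim point, spawns a bullet from the right hand toward it with effects, and decrements ammo.
; A DoOnce and delay limit fire rate, and an empty magazine triggers Reload.
; Reload plays a montage and sound, refilling ammo after a delay; CanShoot works inverted, blocking fire while true.
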(event Custom|Reload
  (bind _wintersolider_ref (Variables|Default|GetWinterSolider%20Ref))
  (bind _wintersolider_ref_2 (Variables|Default|GetWinterSolider%20Ref))
  (if (< (Variables|/Game/Personnage/WinterSoldier/BP_WinterSoldier.BP_WinterSoldier_C|GetMunition _wintersolider_ref) (Variables|/Game/Personnage/WinterSoldier/BP_WinterSoldier.BP_WinterSoldier_C|GetMunitionMax _wintersolider_ref))
    (Variables|Default|SetCan%20Shoot true)
    (Animation|Montage|PlayMontage (Variables|/Script/Engine.Character|GetMesh (Variables|Default|GetWinterSolider%20Ref)) "/Game/Personnage/WinterSoldier/Animation/A_WinterSoldier_Reload_Montage.A_WinterSoldier_Reload_Montage"
      (:then
        (Audio|PlaySound2D "/Engine/EditorSounds/GamePreview/EjectFromPlayer.EjectFromPlayer" 1.0 1.0 0.0 0 0)
        (Utilities|FlowControl|Delay 1.0)
        (Variables|/Game/Personnage/WinterSoldier/BP_WinterSoldier.BP_WinterSoldier_C|SetMunition _wintersolider_ref_2 (Variables|/Game/Personnage/WinterSoldier/BP_WinterSoldier.BP_WinterSoldier_C|GetMunitionMax _wintersolider_ref_2))
        (Variables|Default|SetCan%20Shoot false)))))

(event Custom|Attack
  (bind _wintersolider_ref (Variables|Default|GetWinterSolider%20Ref))
  (bind _wintersolider_ref_2 (Variables|Default|GetWinterSolider%20Ref))
  (bind _mesh (Variables|/Script/Engine.Character|GetMesh _wintersolider_ref))
  (bind _camera (Variables|/Game/Personnage/WinterSoldier/BP_WinterSoldier.BP_WinterSoldier_C|GetCamera _wintersolider_ref_2))
  (bind _returnvalue (Transformation|GetSocketLocation _mesh "Hand_r"))
  (if (not (Variables|Default|GetCan%20Shoot))
    (Utilities|FlowControl|DoOnce false :!label _label
      (:Completed
        (Variables|Default|SetShoot true)
        (bind (_outhit _returnvalue_2) (Collision|LineTraceByChannel (.location (Transformation|GetWorldTransform _camera)) (* (Math|Vector|GetForwardVector _camera) 1e+05) "TraceTypeQuery3" false 0 "None"))
        (Game|SpawnActorfromClass "/Game/Personnage/WinterSoldier/Projectile/BP_WinterBullet.BP_WinterBullet_C" (Math|Transform|MakeTransform (+ _returnvalue (* (Math|Vector|GetForwardVector (Variables|/Game/Personnage/WinterSoldier/BP_WinterSoldier.BP_WinterSoldier_C|GetCamera _wintersolider_ref)) 1e+02)) (Math|Rotator|FindLookatRotation _returnvalue (Math|Vector|SelectVector (.ImpactPoint (Collision|BreakHitResult _outhit)) (.TraceEnd (Collision|BreakHitResult _outhit)) _returnvalue_2)) "1.000000,1.000000,1.000000") "Undefined" "MultiplyWithRoot" 0 0)
        (Effects|SpawnEmitteratLocation "/Game/StarterContent/Particles/P_Explosion.P_Explosion" _returnvalue "0, 0, 0" "0.250000,0.250000,0.250000")
        (Audio|PlaySoundatLocation "/Game/StarterContent/Audio/Explosion01.Explosion01" _returnvalue "0, 0, 0" 1.0 1.0 0.0 0 0 0 0)
        (bind _result (Math|Integer|DecrementInt (Variables|/Game/Personnage/WinterSoldier/BP_WinterSoldier.BP_WinterSoldier_C|GetMunition (Variables|Default|GetWinterSolider%20Ref)))
          (:%20%20
            (Utilities|FlowControl|Delay 0.4)
            (Variables|Default|SetShoot false)
            (if (<= _result 0)
              (CallFunction|Reload)
              (goto _label Reset)
              (else
                (goto _label Reset)))))))))

(event EventBeginPlay
  (bind _asbp_winter_soldier (Utilities|Casting|CastToBP_WinterSoldier (Game|GetPlayerCharacter 0)))
  (Variables|Default|SetWinterSolider%20Ref _asbp_winter_soldier))