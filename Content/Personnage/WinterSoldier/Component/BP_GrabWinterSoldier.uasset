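; Winter Soldier secondary-click grab component: a chargeable ranged pull that snaps a hit Character or Pawn in front of the player.
; Trigger tracks hold time and auto-fires past a limit without updating range, while Completed derives range from the charge, delaying short taps.
; Each shot starts a cooldown and runs a debug-drawn line trace from ahead of the camera toward a hand-socket-based endpoint, then teleports the target.
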(event Custom|Completed
  (bind _holdingtime (Variables|Default|GetHoldingTime))
  ;[0.5791 0.6135 0.724] Secondary click
  (if (not (Variables|Default|GetInCooldown))
    (if (< (Variables|Default|GetHoldingTime) 0.5)
      (Utilities|FlowControl|Delay (- 0.5 (Variables|Default|GetHoldingTime)))
      (Variables|Default|SetRange 1e+01)
      (Development|PrintString "Little charge")
      (Variables|Default|SetInCooldown true)
      (elif (<= _holdingtime 1.0)
        (bind _output_get (Variables|Default|SetRange (Math|Float|Lerp 0.0 2e+01 _holdingtime)))
        (Development|PrintString (Utilities|String|ToString(Float) _output_get))
        (Variables|Default|SetInCooldown true)
        (else
          (bind _output_get_2 (Variables|Default|SetRange 2e+01))
          (Development|PrintString (Utilities|String|ToString(Float) _output_get_2))
          (Variables|Default|SetInCooldown true))))
    (CallFunction|SecondaryCooldown)
    (CallFunction|SecondaryClick)))

(event Custom|SecondaryCooldown
  ;[0.5791 0.6135 0.724] Secondary click
  (Utilities|FlowControl|Delay (Variables|Default|GetCooldownTime))
  (Variables|Default|SetInCooldown false)
  (Development|PrintString "cooldown finish"))

(event Custom|SecondaryClick
  (bind _winter_solider (Variables|Default|GetWinter%20Solider))
  (bind _capsulecomponent (Variables|/Script/Engine.Character|GetCapsuleComponent _winter_solider))
  (bind _camera (Variables|/Game/Personnage/WinterSoldier/BP_WinterSoldier.BP_WinterSoldier_C|GetCamera _winter_solider))
  (bind _returnvalue (Math|Vector|GetForwardVector _camera))
  (bind _returnvalue_2 (Transformation|GetWorldLocation _capsulecomponent))
  (bind _returnvalue_3 (* _returnvalue 5e+01))
  (bind _returnvalue_4 (+ _returnvalue_2 _returnvalue_3))
  ;[0.5791 0.6135 0.724] Secondary click
  (bind _outhit (Collision|LineTraceByChannel (+ (Transformation|GetWorldLocation _camera) (* (Math|Vector|GetForwardVector _camera) 3.5e+02)) (+ (Transformation|GetSocketLocation (Variables|/Script/Engine.Character|GetMesh _winter_solider) "Hand_r") (* (Math|Vector|GetForwardVector _camera) (* (Variables|Default|GetRange) 1e+02))) "TraceTypeQuery3" false 0 "ForDuration"))
  (bind _ascharacter (Utilities|Casting|CastToCharacter (.HitActor (Collision|BreakHitResult _outhit)))
    (:then
      (Transformation|SetActorLocation _ascharacter _returnvalue_4 false false))
    (:CastFailed
      (bind _aspawn (Utilities|Casting|CastToPawn (.HitActor (Collision|BreakHitResult _outhit))))
      (Transformation|SetActorLocation _aspawn _returnvalue_4 false false))))

(event Custom|Trigger
  (params (HoldingTime :type Float%20%28double-precision%29) (WinterSolider :type BP%20Winter%20Soldier%20Object%20Reference))
  ;[0.5791 0.6135 0.724] Secondary click
  (Variables|Default|SetWinter%20Solider WinterSolider)
  (if (not (Variables|Default|GetInCooldown))
    (bind _output_get (Variables|Default|SetHoldingTime HoldingTime))
    (if (> _output_get 4.0)
      (Variables|Default|SetInCooldown true)
      (Development|PrintString "Too much")
      (CallFunction|SecondaryCooldown)
      (CallFunction|SecondaryClick))))

(event EventBeginPlay
  ;[0.5791 0.6135 0.724] Secondary click
)