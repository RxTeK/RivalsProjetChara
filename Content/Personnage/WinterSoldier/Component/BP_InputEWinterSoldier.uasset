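; Input component for the Winter Soldier character's E action, with InputE currently an empty event.
; BeginPlay caches the player character as a Winter Soldier reference.
; An unconnected firing chain traces from the camera and spawns a bullet from the right hand, aimed at the hit point or trace end.
; That chain decrements ammo, then reloads when empty or delays briefly before re-arming its DoOnce.
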(event Custom|InputE)

(event EventBeginPlay
  (bind _asbp_winter_soldier (Utilities|Casting|CastToBP_WinterSoldier (Game|GetPlayerCharacter 0)))
  (Variables|Default|SetWinterSolider%20Ref _asbp_winter_soldier))