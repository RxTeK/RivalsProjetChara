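; Ability component that gives the Winter Soldier player character Tainted Voltage, fired through InputE.
; Each use adds shield, refills munition and spawns a BP_WinterTintedVoltage actor just ahead of the right hand socket.
; A camera line trace orients that actor toward the impact point, or the trace end on a miss.
; A delay-based cooldown flag blocks reuse until CooldownTime elapses.
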(event Custom|CoolDown
  (Utilities|FlowControl|Delay (Variables|Default|GetCooldownTime))
  (Variables|Default|SetInCooldown false))

(event Custom|InputE
  (bind _wintersolider_ref (Variables|Default|GetWinterSolider%20Ref))
  (bind _wintersolider_ref_2 (Variables|Default|GetWinterSolider%20Ref))
  (bind _wintersolider_ref_3 (Variables|Default|GetWinterSolider%20Ref))
  (bind _camera (Variables|/Game/Personnage/WinterSoldier/BP_WinterSoldier.BP_WinterSoldier_C|GetCamera _wintersolider_ref_2))
  (bind _mesh (Variables|/Script/Engine.Character|GetMesh _wintersolider_ref_3))
  (bind _returnvalue (Transformation|GetSocketLocation _mesh "Hand_r"))
  (if (not (Variables|Default|GetInCooldown))
    (Variables|Default|SetInCooldown true)
    (Variables|/Game/Personnage/WinterSoldier/BP_WinterSoldier.BP_WinterSoldier_C|SetShield _wintersolider_ref (+ (Variables|/Game/Personnage/WinterSoldier/BP_WinterSoldier.BP_WinterSoldier_C|GetShield _wintersolider_ref) 4e+01))
    (Variables|/Game/Personnage/WinterSoldier/BP_WinterSoldier.BP_WinterSoldier_C|SetMunition _wintersolider_ref_2 (Variables|/Game/Personnage/WinterSoldier/BP_WinterSoldier.BP_WinterSoldier_C|GetMunitionMax _wintersolider_ref_2))
    (bind (_outhit _returnvalue_2) (Collision|LineTraceByChannel (.location (Transformation|GetWorldTransform _camera)) (* (Math|Vector|GetForwardVector _camera) 1e+05) "TraceTypeQuery3" false 0 "None"))
    (Game|SpawnActorfromClass "/Game/Personnage/WinterSoldier/Projectile/BP_WinterTintedVoltage.BP_WinterTintedVoltage_C" (Math|Transform|MakeTransform (+ _returnvalue (* (Math|Vector|GetForwardVector (Variables|/Game/Personnage/WinterSoldier/BP_WinterSoldier.BP_WinterSoldier_C|GetCamera _wintersolider_ref_3)) 1e+02)) (Math|Rotator|FindLookatRotation _returnvalue (Math|Vector|SelectVector (.ImpactPoint (Collision|BreakHitResult _outhit)) (.TraceEnd (Collision|BreakHitResult _outhit)) _returnvalue_2)) "1.000000,1.000000,1.000000") "Undefined" "MultiplyWithRoot" 0 0)
    (CallFunction|CoolDown)))

(event EventBeginPlay
  (bind _asbp_winter_soldier (Utilities|Casting|CastToBP_WinterSoldier (Game|GetPlayerCharacter 0)))
  (Variables|Default|SetWinterSolider%20Ref _asbp_winter_soldier))