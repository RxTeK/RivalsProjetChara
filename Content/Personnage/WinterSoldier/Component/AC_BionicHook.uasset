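; Winter Soldier ability component for the bionic hook, a charged secondary click that fires a BP_WinterHook.
; Trigger tracks hold time and auto-fires past a limit; Completed converts hold time into hook Range and fires.
; SecondaryClick spawns the hook near the right hand, aimed using a camera line trace.
; A DoOnce grants shield and refills munition once per use, re-armed when the cooldown ends.
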(event Custom|Completed
  (bind _holdingtime (Variables|Default|GetHoldingTime))
  ;[0.5791 0.6135 0.724] Secondary click
  (if (not (Variables|Default|GetInCooldown))
    (if (< (Variables|Default|GetHoldingTime) 0.5)
      (Utilities|FlowControl|Delay (- 0.5 (Variables|Default|GetHoldingTime)))
      (Variables|Default|SetRange 1e+01)
      (Development|PrintString "Little charge")
      (Variables|Default|SetInCooldown true)
      (elif (<= _holdingtime 1.0)
        (bind _output_get (Variables|Default|SetRange (Math|Float|Lerp 0.0 2e+01 _holdingtime)))
        (Development|PrintString (Utilities|String|ToString(Float) _output_get))
        (Variables|Default|SetInCooldown true)
        (else
          (bind _output_get_2 (Variables|Default|SetRange 2e+01))
          (Development|PrintString (Utilities|String|ToString(Float) _output_get_2))
          (Variables|Default|SetInCooldown true))))
    (CallFunction|SecondaryCooldown)
    (CallFunction|SecondaryClick)))

(event Custom|SecondaryClick
  (bind _wintersolider_ref (Variables|Default|GetWinterSolider%20Ref))
  (bind _wintersolider_ref_2 (Variables|Default|GetWinterSolider%20Ref))
  (bind _camera (Variables|/Game/Personnage/WinterSoldier/BP_WinterSoldier.BP_WinterSoldier_C|GetCamera _wintersolider_ref))
  (bind _mesh (Variables|/Script/Engine.Character|GetMesh _wintersolider_ref_2))
  (bind _returnvalue (Transformation|GetSocketLocation _mesh "Hand_r"))
  ;[0.5791 0.6135 0.724] Secondary click
  (bind (_outhit _returnvalue_2) (Collision|LineTraceByChannel (.location (Transformation|GetWorldTransform _camera)) (* (Math|Vector|GetForwardVector _camera) 1e+05) "TraceTypeQuery3" false 0 "None"))
  (Game|SpawnActorfromClass "/Game/Personnage/WinterSoldier/Projectile/BP_WinterHook.BP_WinterHook_C" (Math|Transform|MakeTransform (+ _returnvalue (* (Math|Vector|GetForwardVector (Variables|/Game/Personnage/WinterSoldier/BP_WinterSoldier.BP_WinterSoldier_C|GetCamera _wintersolider_ref_2)) 1.5e+02)) (Math|Rotator|FindLookatRotation _returnvalue (Math|Vector|SelectVector (.ImpactPoint (Collision|BreakHitResult _outhit)) (.TraceEnd (Collision|BreakHitResult _outhit)) _returnvalue_2)) "1.000000,1.000000,1.000000") "Undefined" "MultiplyWithRoot" 0 (Variables|Default|GetRange) 0))

(event Custom|Trigger
  (params (HoldingTime :type Float%20%28double-precision%29))
  (bind _wintersolider_ref (Variables|Default|GetWinterSolider%20Ref))
  (bind _wintersolider_ref_2 (Variables|Default|GetWinterSolider%20Ref))
  ;[0.5791 0.6135 0.724] Secondary click
  (if (not (Variables|Default|GetInCooldown))
    (Utilities|FlowControl|Sequence
      (:then_0
        (bind _output_get (Variables|Default|SetHoldingTime HoldingTime))
        (if (> _output_get 4.0)
          (Variables|Default|SetInCooldown true)
          (Development|PrintString "Too much")
          (CallFunction|SecondaryCooldown)
          (CallFunction|SecondaryClick)))
      (:then_1
        (Utilities|FlowControl|DoOnce false
          (:Completed
            (Variables|/Game/Personnage/WinterSoldier/BP_WinterSoldier.BP_WinterSoldier_C|SetShield _wintersolider_ref_2 (+ (Variables|/Game/Personnage/WinterSoldier/BP_WinterSoldier.BP_WinterSoldier_C|GetShield _wintersolider_ref_2) 4e+01))
            (Variables|/Game/Personnage/WinterSoldier/BP_WinterSoldier.BP_WinterSoldier_C|SetMunition _wintersolider_ref (Variables|/Game/Personnage/WinterSoldier/BP_WinterSoldier.BP_WinterSoldier_C|GetMunitionMax _wintersolider_ref))))))))

(event Custom|SecondaryCooldown
  ;[0.5791 0.6135 0.724] Secondary click
  (Utilities|FlowControl|Delay (Variables|Default|GetCooldownTime))
  (Variables|Default|SetInCooldown false)
  (CallFunction|ResetCooldown)
  (Development|PrintString "cooldown finish"))

(event Custom|Reset%20cooldown
  (bind _wintersolider_ref (Variables|Default|GetWinterSolider%20Ref))
  (bind _wintersolider_ref_2 (Variables|Default|GetWinterSolider%20Ref))
  ;[0.5791 0.6135 0.724] Secondary click
  (Utilities|FlowControl|DoOnce false) ; enters at Reset
)

(event EventBeginPlay
  (bind _asbp_winter_soldier (Utilities|Casting|CastToBP_WinterSoldier (Game|GetPlayerCharacter 0)))
  (Variables|Default|SetWinterSolider%20Ref _asbp_winter_soldier))