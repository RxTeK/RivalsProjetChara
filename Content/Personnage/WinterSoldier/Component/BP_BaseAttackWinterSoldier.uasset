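; BP_BaseAttackWinterSoldier handles the Winter Soldier's basic ranged attack, with limited ammo and reload.
; Attack line-traces from the camera and spawns a BP_WinterBullet near the right-hand socket, aimed at the impact point or trace end.
; A DoOnce throttles fire with a short delay; empty ammo triggers Reload, which refills after a delay.
; The CanShoot flag is inverted: true blocks firing during reload.
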(event Custom|Reload
  (Variables|Default|SetCan%20Shoot true)
  (Utilities|FlowControl|Delay 1.0)
  (Variables|Default|SetMunition (Variables|Default|GetMunitionMax))
  (Variables|Default|SetCan%20Shoot false))

(event Custom|Attack
  (params (WinterSolider :type BP%20Winter%20Soldier%20Object%20Reference))
  (Variables|Default|SetWinter%20Solider WinterSolider)
  (if (not (Variables|Default|GetCan%20Shoot))
    (Utilities|FlowControl|DoOnce false :!label _label
      (:Completed
        (bind (_outhit _returnvalue) (Collision|LineTraceByChannel (.location (Transformation|GetWorldTransform (Variables|/Game/Personnage/WinterSoldier/BP_WinterSoldier.BP_WinterSoldier_C|GetCamera (Variables|Default|GetWinter%20Solider)))) (* (Math|Vector|GetForwardVector (Variables|/Game/Personnage/WinterSoldier/BP_WinterSoldier.BP_WinterSoldier_C|GetCamera (Variables|Default|GetWinter%20Solider))) 1e+05) "TraceTypeQuery3" false 0 "None"))
        (Game|SpawnActorfromClass "/Game/Personnage/WinterSoldier/BP_WinterBullet.BP_WinterBullet_C" (Math|Transform|MakeTransform (+ (Transformation|GetSocketLocation (Variables|/Script/Engine.Character|GetMesh (Variables|Default|GetWinter%20Solider)) "Hand_r") (* (Math|Vector|GetForwardVector (Variables|/Game/Personnage/WinterSoldier/BP_WinterSoldier.BP_WinterSoldier_C|GetCamera (Variables|Default|GetWinter%20Solider))) 1e+02)) (Math|Rotator|FindLookatRotation (Transformation|GetSocketLocation (Variables|/Script/Engine.Character|GetMesh (Variables|Default|GetWinter%20Solider)) "Hand_r") (Math|Vector|SelectVector (.ImpactPoint (Collision|BreakHitResult _outhit)) (.TraceEnd (Collision|BreakHitResult _outhit)) _returnvalue)) "1.000000,1.000000,1.000000") "Undefined" "MultiplyWithRoot" 0 0)
        (bind _result (Math|Integer|DecrementInt (Variables|Default|GetMunition))
          (:%20%20
            (if (<= _result 0)
              (CallFunction|Reload)
              (goto _label Reset)
              (else
                (Utilities|FlowControl|Delay 0.4)
                (goto _label Reset)))))))))