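; BP_Aiming_BW is a component, apparently for the Black Widow character, that toggles aim view on its owning BP_Player.
; On BW_Aim press, a FlipFlop alternates between moving the follow camera to the Aiming point with a new Aiming widget, and restoring it to ResetCam with the widget removed.
; When UltimateON is set, the aim-in branch resets instead.
; The Reloading function is an empty stub.
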(event Input|EnhancedActionEvents|EnhancedInputActionBW_Aim
  (params (ActionValue :type Boolean) (ElapsedSeconds :type Float%20%28double-precision%29) (TriggeredSeconds :type Float%20%28double-precision%29) (InputAction :type Input%20Action%20Object%20Reference :default "/Game/Personnage/Black_Widow_Evan/Input/BW_Aim.BW_Aim"))
  (bind _ref_player_ (Variables|Default|GetRef_player_))
  (bind _followcamera (Variables|/Game/Personnage/ALL/BP_Player.BP_Player_C|GetFollowCamera _ref_player_))
  ;[0 0.2378 1] Aiming
  (:Started
    (Utilities|FlowControl|FlipFlop
      (:A
        (if (Variables|Default|GetUltimateON?)
          (Transformation|SetWorldLocation _followcamera (Transformation|GetWorldLocation (Variables|/Game/Personnage/ALL/BP_Player.BP_Player_C|GetReset%20Cam _ref_player_)) false false :!label _label)
          (Widget|RemovefromParent (Variables|Default|GetAiming_ref))
          (else
            (Transformation|SetWorldLocation _followcamera (Transformation|GetWorldLocation (Variables|/Game/Personnage/ALL/BP_Player.BP_Player_C|GetAiming _ref_player_)) false false)
            (bind _returnvalue (UserInterface|CreateWidget "/Game/Personnage/Black_Widow_Evan/Aiming.Aiming_C"))
            (bind _output_get (Variables|Default|SetAiming_ref _returnvalue))
            (UserInterface|Viewport|AddtoViewport _output_get 0))))
      (:B
        (goto _label)))))

(event EventTick
  (params (DeltaSeconds :type Float%20%28single-precision%29)))

(event EventBeginPlay
  ;[1 0.2761 0] Ref
  (Variables|Default|SetRef_player_ (.AsBP%20Player (Utilities|Casting|CastToBP_Player (Components|GetOwner)))))

(fn Reloading)