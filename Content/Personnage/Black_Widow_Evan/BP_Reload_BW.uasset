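; Reload logic for the Black Widow character, owned by BP_Player, that refills its magazine.
; The BW_Reload input starts a timer, and when it fires the magazine is topped up to its eight-round cap after a four-second delay.
; The owning player is cached on BeginPlay but not used afterward, and the Reloading function is an empty stub.
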(event Custom|Reload
  ;[0 1 0.8751] Reload
  (Utilities|Time|SetTimerbyEvent (delegate Custom|Delayy) 4.0))

(event Custom|Delayy
  ;[0 1 0.8751] Reload
  (Variables|Default|SetMagazine (Math|Integer|Clamp(Integer) (+ (Variables|Default|GetMagazine) 8) 0 8)))

(event Input|EnhancedActionEvents|EnhancedInputActionBW_Reload
  (params (ActionValue :type Boolean) (ElapsedSeconds :type Float%20%28double-precision%29) (TriggeredSeconds :type Float%20%28double-precision%29) (InputAction :type Input%20Action%20Object%20Reference :default "/Game/Personnage/Black_Widow_Evan/Input/BW_Reload.BW_Reload"))
  ;[0 1 0.8751] Reload
  (:Started
    (CallFunction|Reload)))

(event EventTick
  (params (DeltaSeconds :type Float%20%28single-precision%29)))

(event EventBeginPlay
  ;[1 0.2761 0] Ref
  (Variables|Default|SetRef_player_ (.AsBP%20Player (Utilities|Casting|CastToBP_Player (Components|GetOwner)))))

(fn Reloading)