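; Sprint component for the Black Widow player, driven by the BW_run input and the owner's tagged BP_Energy_BW component.
; Pressing while moving and not flying gives a short launch along the velocity, given enough energy.
; Holding with enough energy raises walk speed and jump velocity, and a looping timer drains EnergyMax each second.
; Releasing, low energy or depletion calls the component's Energy function, with CanRun and CanEnergise flags gating re-triggering.
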(event Custom|running
  (bind _ref_player_ (Variables|Default|GetRef_player_))
  (bind _returnvalue (Class|Actor|FindComponentbyTag _ref_player_ "/Game/Personnage/Black_Widow_Evan/BP_Energy_BW.BP_Energy_BW_C" "Energy"))
  ;[0.03439 1 0.311] Running
  (Variables|/Game/Personnage/Black_Widow_Evan/BP_Energy_BW.BP_Energy_BW_C|SetEnergy_max _returnvalue (Math|Float|Clamp(Float) (- (Variables|/Game/Personnage/Black_Widow_Evan/BP_Energy_BW.BP_Energy_BW_C|GetEnergy_max _returnvalue) 12.0) 0.0 1.2e+02))
  (if (and (Utilities|Time|IsValidTimerHandle (Variables|Default|GetNewVar_0)) (<= 0.0 0.0))
    (Variables|Default|SetCanEnergise? true)
    (Default|Energy (Class|Actor|FindComponentbyTag (Variables|Default|GetRef_player_) "/Game/Personnage/Black_Widow_Evan/BP_Energy_BW.BP_Energy_BW_C" "Energy"))
    (Utilities|Time|ClearandInvalidateTimerbyHandle (Variables|Default|GetNewVar_0))))

(event Custom|Run
  (bind _ref_player_ (Variables|Default|GetRef_player_))
  (bind _charactermovement (Variables|/Script/Engine.Character|GetCharacterMovement _ref_player_))
  ;[0.03439 1 0.311] Running
  (Variables|/Script/Engine.CharacterMovementComponent|SetMaxWalkSpeed _charactermovement 798.0)
  (Variables|/Script/Engine.CharacterMovementComponent|SetJumpZVelocity _charactermovement 1.5e+03)
  (bind _returnvalue (Utilities|Time|SetTimerbyEvent (delegate Custom|running) 1.0 true false -0.2))
  (Variables|Default|SetNewVar_0 _returnvalue))

(event Input|EnhancedActionEvents|EnhancedInputActionBW_run
  (params (ActionValue :type Boolean) (ElapsedSeconds :type Float%20%28double-precision%29) (TriggeredSeconds :type Float%20%28double-precision%29) (InputAction :type Input%20Action%20Object%20Reference :default "/Game/Personnage/Black_Widow_Evan/Input/BW_run.BW_run"))
  (bind _ref_player_ (Variables|Default|GetRef_player_))
  (bind _ref_player__2 (Variables|Default|GetRef_player_))
  (bind _returnvalue (Class|Actor|FindComponentbyTag _ref_player__2 "/Game/Personnage/Black_Widow_Evan/BP_Energy_BW.BP_Energy_BW_C" "Energy"))
  (bind _charactermovement (Variables|/Script/Engine.Character|GetCharacterMovement _ref_player_))
  (bind _velocity (Variables|/Script/Engine.MovementComponent|GetVelocity _charactermovement))
  (bind _energy_max (Variables|/Game/Personnage/Black_Widow_Evan/BP_Energy_BW.BP_Energy_BW_C|GetEnergy_max _returnvalue))
  (bind (_x _y) (Math|Vector|BreakVector _velocity))
  (bind _returnvalue_2 (Math|Vector|Normalize (Math|Vector|MakeVector _x _y 0.0) 0.0))
  (bind _returnvalue_3 (* _returnvalue_2 2e+02))
  (bind (_x_2 _y_2) (Math|Vector|BreakVector _returnvalue_3))
  ;[1 0.8158 0] Run
  (:Started
    (if (not (Variables|Default|GetIsOnFly?))
      (if (and (< 0.0 (Math|Vector|VectorLengthXY _velocity)) (> _energy_max 24.0))
        (Character|LaunchCharacter (Variables|Default|GetRef_player_) (Math|Vector|MakeVector _x_2 _y_2 0.0) false false))))
  (:Ongoing
    (if (not (Variables|Default|GetIsOnFly?))
      (if (<= _energy_max 3e+01)
        (if (Variables|Default|GetCanEnergise?)
          (Variables|Default|SetCanEnergise? false)
          (Default|Energy (Class|Actor|FindComponentbyTag (Variables|Default|GetRef_player_) "/Game/Personnage/Black_Widow_Evan/BP_Energy_BW.BP_Energy_BW_C" "Energy")))
        (elif (Variables|/Game/Personnage/Black_Widow_Evan/BP_Energy_BW.BP_Energy_BW_C|GetCanRun? _returnvalue)
          (Variables|/Game/Personnage/Black_Widow_Evan/BP_Energy_BW.BP_Energy_BW_C|SetCanRun? _returnvalue false)
          (CallFunction|Run)))))
  (:Canceled
    (Utilities|Time|ClearandInvalidateTimerbyHandle (Variables|Default|GetNewVar_0) :!label _label)
    (Default|Energy _returnvalue)
    (if (not (<= _energy_max 3e+01))
      (Variables|/Game/Personnage/Black_Widow_Evan/BP_Energy_BW.BP_Energy_BW_C|SetCanRun? _returnvalue true)))
  (:Completed
    (goto _label)))

(event EventTick
  (params (DeltaSeconds :type Float%20%28single-precision%29))
  ;[1 0.8158 0] Run
)

(event EventBeginPlay
  ;[1 0.2761 0] Ref
  (Variables|Default|SetRef_player_ (.AsBP%20Player (Utilities|Casting|CastToBP_Player (Components|GetOwner)))))

(fn Reloading)