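; Player component that handles the Black Widow character's shoot input, caching its BP_Player owner on BeginPlay.
; Pressing shoot calls UltimateShoot on the ultimate component when the aiming component reports UltimateON, otherwise fires the tagged damage-falloff component, limited by a one-second timer cooldown.
; Releasing or canceling during the ultimate clears its Ultiaugment timer and launches the ultimate.
; The Reloading function is an empty stub.
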(event Custom|Delay
  ;[1 0 0.2327] Shoot
  (Variables|Default|SetDelaytest? false))

(event Input|EnhancedActionEvents|EnhancedInputActionBW_Shoot
  (params (ActionValue :type Vector%202D%20Structure) (ElapsedSeconds :type Float%20%28double-precision%29) (TriggeredSeconds :type Float%20%28double-precision%29) (InputAction :type Input%20Action%20Object%20Reference :default "/Game/Personnage/Black_Widow_Evan/Input/BW_Shoot.BW_Shoot"))
  (bind _refplayer (Variables|Default|GetRefplayer))
  (bind _refplayer_2 (Variables|Default|GetRefplayer))
  (bind _returnvalue (Actor|GetComponentbyClass _refplayer "/Game/Personnage/Black_Widow_Evan/BP_Ultimate_Bw.BP_Ultimate_Bw_C"))
  (bind _returnvalue_2 (Actor|GetComponentbyClass _refplayer_2 "/Game/Personnage/Black_Widow_Evan/BP_Aiming_BW.BP_Aiming_BW_C"))
  (bind _ultimateon_ (Variables|/Game/Personnage/Black_Widow_Evan/BP_Aiming_BW.BP_Aiming_BW_C|GetUltimateON? _returnvalue_2))
  ;[1 0 0.2327] Shoot
  (:Started
    (if _ultimateon_
      (Default|UltimateShoot _returnvalue)
      (elif (not (Variables|Default|GetDelaytest?))
        (Default|Shoot (Class|Actor|FindComponentbyTag (Variables|Default|GetRefplayer) "/Game/Personnage/Black_Widow_Evan/BP_Damagefalloff_BW.BP_Damagefalloff_BW_C" "Damagefall"))
        (Variables|Default|SetDelaytest? true)
        (Utilities|Time|SetTimerbyEvent (delegate Custom|Delay) 1.0))))
  (:Canceled
    (if _ultimateon_ :!label _label
      (Utilities|Time|ClearandInvalidateTimerbyHandle (Variables|/Game/Personnage/Black_Widow_Evan/BP_Ultimate_Bw.BP_Ultimate_Bw_C|Getultiaugment _returnvalue))
      (Default|LaunchUlti _returnvalue)))
  (:Completed
    (goto _label)))

(event EventTick
  (params (DeltaSeconds :type Float%20%28single-precision%29)))

(event EventBeginPlay
  ;[0 0.2378 1] Ref
  (Variables|Default|SetRefplayer (.AsBP%20Player (Utilities|Casting|CastToBP_Player (Components|GetOwner)))))

(fn Reloading)