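; Black Widow spell component for the player, giving an input-triggered melee-range area knockback.
; The input plays the spell montage and immediately runs a debug-drawn sphere trace around the player.
; A hit BP_Dummy is launched along a fixed world-space vector and triggers the HUD hit marker.
; The Attack flag re-arms after a delay only on a hit, so a miss leaves the spell locked; Reloading is empty.
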(event Input|EnhancedActionEvents|EnhancedInputActionBW_spell1
  (params (ActionValue :type Vector%202D%20Structure) (ElapsedSeconds :type Float%20%28double-precision%29) (TriggeredSeconds :type Float%20%28double-precision%29) (InputAction :type Input%20Action%20Object%20Reference :default "/Game/Personnage/Black_Widow_Evan/Input/BW_spell1.BW_spell1"))
  (bind _refplayer (Variables|Default|GetRefplayer))
  (:Started
    (if (Variables|Default|Getattack)
      (Variables|Default|Setattack false)
      (Animation|Montage|PlayMontage (Variables|/Script/Engine.Character|GetMesh (Variables|Default|GetRefplayer)) "/Game/Personnage/Black_Widow_Evan/ExportBWAnim/RetargetedAnim/bw_spell_montage.bw_spell_montage" 0.8
        (:then
          (bind _outhit (Collision|SphereTraceByChannel (Transformation|GetWorldLocation (Variables|/Script/Engine.Actor|GetRootComponent _refplayer)) (Transformation|GetWorldLocation (Variables|/Script/Engine.Actor|GetRootComponent _refplayer)) 2.5e+02 "TraceTypeQuery3" false 0 "ForDuration"))
          (bind _asbp_dummy (Utilities|Casting|CastToBP_Dummy (.HitActor (Collision|BreakHitResult _outhit))))
          (Character|LaunchCharacter _asbp_dummy "0.000000,500.000000,500.000000" false false)
          (Default|SetHitMarker (Variables|/Game/Personnage/ALL/BP_Player.BP_Player_C|GetHUD%20REF (Variables|Default|GetRefplayer)))
          (Utilities|FlowControl|Delay 1e+01)
          (Variables|Default|Setattack true))))))

(event EventTick
  (params (DeltaSeconds :type Float%20%28single-precision%29)))

(event EventBeginPlay
  ;[0 0.2378 1] Ref
  (Variables|Default|SetRefplayer (.AsBP%20Player (Utilities|Casting|CastToBP_Player (Components|GetOwner)))))

(fn Reloading)