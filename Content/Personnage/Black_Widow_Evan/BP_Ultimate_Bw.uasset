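; Black Widow's chargeable ultimate ability, attached to the player and driven by the BW_ultimate input.
; At full Ultimate, the input switches BP_Aiming_BW to ultimate mode and moves the follow camera to the ultimate viewpoint.
; UltimateShoot starts a looping timer that raises clamped damage, explosion range and globule count.
; Launch_ulti spawns an actor from the camera transform with those stats, then resets camera, stats and energy; Tick prints debug values.
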(event Custom|Launch_ulti
  (bind _ref_player_ (Variables|Default|GetRef_player_))
  ;[0 1 0.4011] Launch_Ultime
  (Utilities|FlowControl|DoOnce false :!label _label
    (:Completed
      (Variables|/Game/Personnage/Black_Widow_Evan/BP_Aiming_BW.BP_Aiming_BW_C|SetUltimateON? (Actor|GetComponentbyClass (Variables|Default|GetRef_player_) "/Game/Personnage/Black_Widow_Evan/BP_Aiming_BW.BP_Aiming_BW_C") false)
      (Game|SpawnActorfromClass "/Game/Personnage/Black_Widow_Evan/BP_bw_ult_pro.BP_bw_ult_pro_C" (Transformation|GetWorldTransform (Variables|/Game/Personnage/ALL/BP_Player.BP_Player_C|GetFollowCamera (Variables|Default|GetRef_player_))) "Undefined" "MultiplyWithRoot" 0 (Variables|Default|GetDammage_Ultimate) (Variables|Default|GetExplosionRange) (Variables|Default|GetNb_of_globule) 0)
      (Transformation|SetWorldLocation (Variables|/Game/Personnage/ALL/BP_Player.BP_Player_C|GetFollowCamera _ref_player_) (Transformation|GetWorldLocation (Variables|/Game/Personnage/ALL/BP_Player.BP_Player_C|GetReset%20Cam _ref_player_)) false false)
      (Variables|Default|SetExplosionRange 5.6)
      (Variables|Default|SetNb_of_globule 7.0)
      (Variables|/Game/Personnage/ALL/BP_Player.BP_Player_C|SetEnergy (Variables|Default|GetRef_player_) 0.0)
      (Variables|Default|SetDammage_Ultimate 1.2e+02)
      (Variables|Default|SetUltimate%25 0.0)
      (goto _label Reset))))

(event Custom|UltimateShoot
  ;[1 0 0.96] Charge
  (bind _returnvalue (Utilities|Time|SetTimerbyEvent (delegate Custom|charge) 0.6 true false -0.6))
  (Variables|Default|Setultiaugment _returnvalue))

(event Custom|charge
  ;[1 0 0.96] Charge
  (Variables|Default|SetExplosionRange (Math|Float|Clamp(Float) (+ (Variables|Default|GetExplosionRange) 6e+01) 5.6e+02 8e+02))
  (Variables|Default|SetNb_of_globule (Math|Float|Clamp(Float) (+ (Variables|Default|GetNb_of_globule) 2.0) 7.0 2e+01))
  (Variables|Default|SetDammage_Ultimate (Math|Float|Clamp(Float) (+ (Variables|Default|GetDammage_Ultimate) 1e+01) 1.2e+02 1.7e+02)))

(event Input|EnhancedActionEvents|EnhancedInputActionBW_ultimate
  (params (ActionValue :type Boolean) (ElapsedSeconds :type Float%20%28double-precision%29) (TriggeredSeconds :type Float%20%28double-precision%29) (InputAction :type Input%20Action%20Object%20Reference :default "/Game/Personnage/Black_Widow_Evan/Input/BW_ultimate.BW_ultimate"))
  (bind _ref_player_ (Variables|Default|GetRef_player_))
  (bind _returnvalue (Actor|GetComponentbyClass _ref_player_ "/Game/Personnage/Black_Widow_Evan/BP_Aiming_BW.BP_Aiming_BW_C"))
  ;[1 0 0.96] Charge
  (:Started
    (if (== (Variables|Default|GetUltimate%25) 1e+02)
      (Widget|RemovefromParent (Variables|/Game/Personnage/Black_Widow_Evan/BP_Aiming_BW.BP_Aiming_BW_C|GetAiming_ref _returnvalue))
      (Variables|/Game/Personnage/Black_Widow_Evan/BP_Aiming_BW.BP_Aiming_BW_C|SetUltimateON? _returnvalue true)
      (Transformation|SetWorldLocation (Variables|/Game/Personnage/ALL/BP_Player.BP_Player_C|GetFollowCamera (Variables|Default|GetRef_player_)) (Transformation|GetWorldLocation (Variables|/Game/Personnage/ALL/BP_Player.BP_Player_C|GetUltimate (Variables|Default|GetRef_player_))) false false))))

(event EventTick
  (params (DeltaSeconds :type Float%20%28single-precision%29))
  (Development|PrintString (Utilities|String|ToString(Float) (Variables|Default|GetDammage_Ultimate)) true true "(R=0.000000,G=0.660000,B=1.000000,A=1.000000)" 0.0)
  (Development|PrintString (Utilities|String|ToString(Float) (Variables|Default|GetExplosionRange)) true true "(R=0.000000,G=0.660000,B=1.000000,A=1.000000)" 0.0)
  (Development|PrintString (Utilities|String|ToString(Float) (Variables|Default|GetNb_of_globule)) true true "(R=0.000000,G=0.660000,B=1.000000,A=1.000000)" 0.0)
  (Development|PrintString "Stat Ultime :" true true "(R=0.000000,G=0.660000,B=1.000000,A=1.000000)" 0.0))

(event EventBeginPlay
  ;[1 0.2761 0] Ref
  (Variables|Default|SetRef_player_ (.AsBP%20Player (Utilities|Casting|CastToBP_Player (Components|GetOwner)))))

(fn Reloading)