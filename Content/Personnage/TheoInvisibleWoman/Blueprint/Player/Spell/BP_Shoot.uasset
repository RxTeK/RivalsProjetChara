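; Boomerang-style projectile for the Invisible Woman's orb shot, damaging enemy dummies it overlaps.
; A looping timer watches the distance to the player; exceeding range, or overlapping anything other than a dummy or the player, starts the return.
; The return uses a per-frame timer to steer velocity back toward the player.
; Touching the player while returning re-enables shooting on the orb projection and destroys the projectile.
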(event OnComponentBeginOverlap(Sphere)
  (params (OverlappedComponent :type Primitive%20Component%20Object%20Reference) (OtherActor :type Actor%20Object%20Reference) (OtherComp :type Primitive%20Component%20Object%20Reference) (OtherBodyIndex :type Integer) (bFromSweep :type Boolean) (SweepResult :type Hit%20Result%20Structure%20%28by%20ref%29))
  (bind _asbp_dummy (Utilities|Casting|CastToBP_Dummy OtherActor)
    (:then
      (if (Utilities|Select :Index (Variables|/Game/Personnage/Dummy/BP_Dummy.BP_Dummy_C|GetDummyType _asbp_dummy) :NewEnumerator0 true :NewEnumerator1 false)
        (Game|Damage|ApplyDamage _asbp_dummy (Variables|Default|GetDammage) 0 0)
        (Development|PrintString "Ennemy")))
    (:CastFailed
      (if (not (Variables|Default|GetReturn))
        (Utilities|Casting|CastToBP_InvisibleWoman OtherActor
          (:CastFailed
            (CallFunction|ReturnProjectile)))
        (else
          (Utilities|Casting|CastToBP_InvisibleWoman OtherActor)
          (Variables|/Game/Personnage/TheoInvisibleWoman/Blueprint/Player/Spell/BP_OrbProjection.BP_OrbProjection_C|SetCanShoot? (Variables|/Game/Personnage/TheoInvisibleWoman/Blueprint/Player/BP_InvisibleWoman.BP_InvisibleWoman_C|GetBP_OrbProjection (Variables|Default|GetPlayerRef)) true)
          (Actor|DestroyActor))))))

(event Custom|VerifDistance
  (bind _output_get (Variables|Default|SetLocation (Transformation|GetActorLocation)))
  (if (> (Math|Vector|Distance(Vector) (Transformation|GetActorLocation (Variables|Default|GetPlayerRef)) _output_get) 3e+03)
    (Utilities|FlowControl|DoOnce false
      (:Completed
        (CallFunction|ReturnProjectile)
        (Utilities|Time|ClearandInvalidateTimerbyHandle (Variables|Default|GetTimerVerifDistance))))))

(event Custom|ReturnProjectile
  (Utilities|Time|SetTimerbyEvent (EventDispatchers|CreateEvent :!event Custom|FollowPlayer) (Utilities|Time|GetWorldDeltaSeconds) true))

(event Custom|FollowPlayer
  (Variables|Default|SetReturn true)
  (Transformation|SetActorRotation (Math|Interpolation|RInterpTo (Transformation|GetActorRotation) (Math|Rotator|FindLookatRotation (Transformation|GetActorLocation) (Transformation|GetActorLocation (Variables|Default|GetPlayerRef))) (Utilities|Time|GetWorldDeltaSeconds) 2e+02))
  (Variables|/Script/Engine.MovementComponent|SetVelocity (Variables|Default|GetProjectileMovement) (* (Transformation|GetActorForwardVector) 4e+03)))

(event EventBeginPlay
  (Variables|Default|SetReturn false)
  (Components|Activation|Activate (Variables|Default|GetProjectileMovement) false)
  (bind _returnvalue (Utilities|Time|SetTimerbyEvent (EventDispatchers|CreateEvent :!event Custom|VerifDistance) (Utilities|Time|GetWorldDeltaSeconds) true))
  (Variables|Default|SetTimerVerifDistance _returnvalue))

(fn ConstructionScript)