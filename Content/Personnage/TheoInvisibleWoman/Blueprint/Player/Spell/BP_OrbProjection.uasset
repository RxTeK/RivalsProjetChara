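; Orb projection spell component for BP_Player that fires BP_IwShoot projectiles on input, ending invisibility and shaking the camera.
; Each shot decrements ammo, updates the HUD and instantly resets ammo to max at zero, while a FlipFlop alternates two montages.
; A camera trace sets the aim point for the projectile spawned at the right hand.
; A CanShoot flag gates firing until DelayShoot re-enables it after a short delay.
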(event Custom|DelayShoot
  (Utilities|FlowControl|Delay 0.1)
  (Variables|Default|SetCanShoot? true))

(event Input|EnhancedActionEvents|EnhancedInputActionIA_OrbProjectionIW
  (params (ActionValue :type Boolean) (ElapsedSeconds :type Float%20%28double-precision%29) (TriggeredSeconds :type Float%20%28double-precision%29) (InputAction :type Input%20Action%20Object%20Reference :default "/Game/Personnage/TheoInvisibleWoman/Input/IA_OrbProjectionIW.IA_OrbProjectionIW"))
  (bind _returnvalue (Components|GetOwner))
  (bind _character_ref (Variables|Default|GetCharacter%20Ref))
  (bind _character_ref_2 (Variables|Default|GetCharacter%20Ref))
  (bind _character_ref_3 (Variables|Default|GetCharacter%20Ref))
  (bind _asbp_player (Utilities|Casting|CastToBP_Player _returnvalue))
  (bind _mesh (Variables|/Script/Engine.Character|GetMesh _character_ref_3))
  (bind _max_ammo (Variables|/Game/Personnage/ALL/BP_Player.BP_Player_C|GetMax%20Ammo _character_ref))
  (bind _returnvalue_2 (Transformation|GetSocketLocation _mesh "hand_r"))
  (bind _followcamera (Variables|/Game/Personnage/ALL/BP_Player.BP_Player_C|GetFollowCamera _asbp_player))
  (bind _returnvalue_3 (Transformation|GetWorldLocation _followcamera))
  (:Started
    (if (Variables|Default|GetCanShoot?)
      (Variables|Default|SetCanShoot? false)
      (bind _result (Math|Float|DecrementFloat (Variables|/Game/Personnage/ALL/BP_Player.BP_Player_C|GetAmmo _character_ref))
        (:%20%20
          (Default|SetMunitions (Variables|/Game/Personnage/ALL/BP_Player.BP_Player_C|GetHUD%20REF _character_ref) (Math|Float|Clamp(Float) _result 0.0 _max_ammo) _max_ammo)
          (if (== (Math|Float|Clamp(Float) _result 0.0 _max_ammo) 0.0)
            (Variables|/Game/Personnage/ALL/BP_Player.BP_Player_C|SetAmmo _character_ref _max_ammo))
          (bind _isa (Utilities|FlowControl|FlipFlop)
            (:A
              _)
            (:B
              _))
          (Variables|Default|SetIs%20A _isa)
          (Default|InvicibleOff (Actor|GetComponentbyClass _character_ref_2 "/Game/Personnage/TheoInvisibleWoman/Blueprint/Player/Spell/BP_Invicibility.BP_Invicibility_C"))
          (Animation|Montage|PlayMontage (Variables|/Script/Engine.Character|GetMesh _character_ref_2) (Utilities|Select :Index (Math|Conversions|ToInteger(Boolean) _isa) :Option%200 "/Game/Personnage/TheoInvisibleWoman/Animation/Anim/SK_Mannequin_Sequence_Montage.SK_Mannequin_Sequence_Montage" :Option%201 "/Game/Personnage/TheoInvisibleWoman/Animation/Anim/AnimIW_SK_1050_1050001_105011_Primary_02_Montage.AnimIW_SK_1050_1050001_105011_Primary_02_Montage")
            (:then
              (bind _outhit (Collision|LineTraceByChannel _returnvalue_3 (+ _returnvalue_3 (* (Math|Vector|GetForwardVector _followcamera) 3e+03)) "TraceTypeQuery2" false 0 "None"))
              (Game|SpawnActorfromClass "/Game/Personnage/TheoInvisibleWoman/Blueprint/Player/Spell/BP_IwShoot.BP_IwShoot_C" (Math|Transform|MakeTransform _returnvalue_2 (Math|Rotator|FindLookatRotation _returnvalue_2 (Math|Vector|SelectVector (.TraceEnd (Collision|BreakHitResult _outhit)) (.ImpactPoint (Collision|BreakHitResult _outhit)) (Utilities|Operators|EqualEqual :A (.ImpactPoint (Collision|BreakHitResult _outhit))))) "1.000000,1.000000,1.000000") "Undefined" "MultiplyWithRoot" 0 (Variables|Default|GetCharacter%20Ref) 0)
              (Camera|PlayWorldCameraShake "/Game/Personnage/TheoInvisibleWoman/Blueprint/Shake/CS_ShootIW.CS_ShootIW_C" (Transformation|GetActorLocation (Variables|Default|GetCharacter%20Ref)) 5e+02 2e+03))))))))

(event EventBeginPlay
  (Variables|Default|SetCharacter%20Ref (.AsBP%20Player (Utilities|Casting|CastToBP_Player (Components|GetOwner)))))