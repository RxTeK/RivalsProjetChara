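; Player ability component for Invisible Woman's Psionic Vortex, which fires an orb projectile on input.
; Each press alternates between two strike montages through a FlipFlop.
; A camera-forward line trace picks the aim point, and BP_IwOrb spawns at the spine socket rotated toward it.
; Firing also plays a world camera shake and calls InvicibleOff on the owner's BP_Invicibility component.
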(event Input|EnhancedActionEvents|EnhancedInputActionIA_PsionicVortexIW
  (params (ActionValue :type Boolean) (ElapsedSeconds :type Float%20%28double-precision%29) (TriggeredSeconds :type Float%20%28double-precision%29) (InputAction :type Input%20Action%20Object%20Reference :default "/Game/Personnage/TheoInvisibleWoman/Input/IA_PsionicVortexIW.IA_PsionicVortexIW"))
  (bind _returnvalue (Components|GetOwner))
  (bind _character_ref (Variables|Default|GetCharacter%20Ref))
  (bind _asbp_player (Utilities|Casting|CastToBP_Player _returnvalue))
  (bind _mesh (Variables|/Script/Engine.Character|GetMesh _character_ref))
  (bind _returnvalue_2 (Transformation|GetSocketLocation _mesh "spine_04"))
  (bind _followcamera (Variables|/Game/Personnage/ALL/BP_Player.BP_Player_C|GetFollowCamera _asbp_player))
  (bind _returnvalue_3 (Transformation|GetWorldLocation _followcamera))
  (:Started
    (bind _isa (Utilities|FlowControl|FlipFlop)
      (:A
        _)
      (:B
        _))
    (Animation|Montage|PlayMontage (Variables|/Script/Engine.Character|GetMesh (Variables|Default|GetCharacter%20Ref)) (select _isa "/Game/Personnage/TheoInvisibleWoman/Animation/Anim/AnimIW_SK_1050_1050001_105031_PsionicStrike_01_Montage.AnimIW_SK_1050_1050001_105031_PsionicStrike_01_Montage" "/Game/Personnage/TheoInvisibleWoman/Animation/Anim/AnimIW_SK_1050_1050001_105031_PsionicStrike_02_Montage.AnimIW_SK_1050_1050001_105031_PsionicStrike_02_Montage")
      (:then
        (bind _outhit (Collision|LineTraceByChannel _returnvalue_3 (+ _returnvalue_3 (* (Math|Vector|GetForwardVector _followcamera) 3e+03)) "TraceTypeQuery2" false 0 "None"))
        (Game|SpawnActorfromClass "/Game/Personnage/TheoInvisibleWoman/Blueprint/Player/Spell/BP_IwOrb.BP_IwOrb_C" (Math|Transform|MakeTransform _returnvalue_2 (Math|Rotator|FindLookatRotation _returnvalue_2 (Math|Vector|SelectVector (.TraceEnd (Collision|BreakHitResult _outhit)) (.ImpactPoint (Collision|BreakHitResult _outhit)) (Utilities|Operators|EqualEqual :A (.ImpactPoint (Collision|BreakHitResult _outhit))))) "1.000000,1.000000,1.000000") "Undefined" "MultiplyWithRoot" 0 (Variables|Default|GetCharacter%20Ref) 0)
        (Camera|PlayWorldCameraShake "/Game/Personnage/TheoInvisibleWoman/Blueprint/Shake/CS_ShootIW.CS_ShootIW_C" (Transformation|GetActorLocation (Variables|Default|GetCharacter%20Ref)) 5e+02 2e+03)
        (Default|InvicibleOff (Actor|GetComponentbyClass (Variables|Default|GetCharacter%20Ref) "/Game/Personnage/TheoInvisibleWoman/Blueprint/Player/Spell/BP_Invicibility.BP_Invicibility_C"))))))

(event EventBeginPlay
  (Variables|Default|SetCharacter%20Ref (.AsCharacter (Utilities|Casting|CastToCharacter (Components|GetOwner)))))