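; Player spell component that gives its owning Character a boosted double jump tied to invisibility.
; Jump input while falling fires a DoOnce that allows two jumps, raises jump Z velocity, doubles current velocity and calls InvisibleOn on the tagged invincibility component.
; A looping per-frame timer polls for landing, then clears itself, removes the jump boost and resets the DoOnce.
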(event Custom|OnGround?
  (bind _characterref (Variables|Default|GetCharacterRef))
  (bind _charactermovement (Variables|/Script/Engine.Character|GetCharacterMovement _characterref))
  (bind _output_get (Variables|Default|SetIs%20Falling? (AI|Components|NavMovement|IsFalling _charactermovement)))
  (if (not _output_get)
    (Utilities|Time|ClearandInvalidateTimerbyHandle (Variables|Default|GetTimer))
    (Variables|Default|SetDoubleJumpOn false)
    (Variables|/Script/Engine.CharacterMovementComponent|SetJumpZVelocity _charactermovement (- (Variables|/Script/Engine.CharacterMovementComponent|GetJumpZVelocity _charactermovement) (Variables|Default|GetBoost2Jump)))
    (Utilities|FlowControl|DoOnce false) ; enters at Reset
  ))

(event Input|EnhancedActionEvents|EnhancedInputActionIA_JumpIW
  (params (ActionValue :type Boolean) (ElapsedSeconds :type Float%20%28double-precision%29) (TriggeredSeconds :type Float%20%28double-precision%29) (InputAction :type Input%20Action%20Object%20Reference :default "/Game/Personnage/TheoInvisibleWoman/Input/IA_JumpIW.IA_JumpIW"))
  (:Started
    (bind _output_get (Variables|Default|SetCharacterRef (.AsCharacter (Utilities|Casting|CastToCharacter (Components|GetOwner)))))
    (if (AI|Components|NavMovement|IsFalling (Variables|/Script/Engine.Character|GetCharacterMovement _output_get))
      (Variables|Default|SetDoubleJumpOn true)
      (bind _returnvalue (Utilities|Time|SetTimerbyEvent (EventDispatchers|CreateEvent :!event Custom|OnGround?) (Utilities|Time|GetWorldDeltaSeconds) true))
      (Variables|Default|SetTimer _returnvalue)
      (Utilities|FlowControl|DoOnce false
        (:Completed
          (Variables|/Script/Engine.Character|SetJumpMaxCount (Variables|Default|GetCharacterRef) 2)
          (Variables|/Script/Engine.CharacterMovementComponent|SetJumpZVelocity (Variables|/Script/Engine.Character|GetCharacterMovement (Variables|Default|GetCharacterRef)) (+ (Variables|/Script/Engine.CharacterMovementComponent|GetJumpZVelocity (Variables|/Script/Engine.Character|GetCharacterMovement (Variables|Default|GetCharacterRef))) (Variables|Default|GetBoost2Jump)))
          (Variables|/Script/Engine.MovementComponent|SetVelocity (Variables|/Script/Engine.Character|GetCharacterMovement (Variables|Default|GetCharacterRef)) (* (Variables|/Script/Engine.MovementComponent|GetVelocity (Variables|/Script/Engine.Character|GetCharacterMovement (Variables|Default|GetCharacterRef))) 2.0))
          (Default|Invisibleon (Class|Actor|FindComponentbyTag (Variables|Default|GetCharacterRef) "/Game/Personnage/TheoInvisibleWoman/Blueprint/Player/Spell/BP_Invicibility.BP_Invicibility_C" "Invicibility")))))))