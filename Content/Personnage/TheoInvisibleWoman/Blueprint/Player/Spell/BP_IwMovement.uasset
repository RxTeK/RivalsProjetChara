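; Movement component for the Invisible Woman player character, handling look, move and jump through Enhanced Input actions.
; It casts its owner to Character on BeginPlay, then feeds yaw, pitch and control-rotation-relative movement to it.
; Starting a jump also starts a per-frame looping timer, apparently driving JumpShake, which uses IsFalling and a DoOnce to play a landing camera shake and clear the timer.
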(event Custom|JumpShake
  (if (AI|Components|NavMovement|IsFalling (Variables|/Script/Engine.Character|GetCharacterMovement (Variables|Default|GetPlayer)))
    (goto _label Reset)
    (else
      (Utilities|FlowControl|DoOnce false :!label _label
        (:Completed
          (Camera|PlayWorldCameraShake "/Game/Personnage/TheoInvisibleWoman/Blueprint/Shake/CS_ShootIW.CS_ShootIW_C" (Transformation|GetActorLocation (Variables|Default|GetPlayer)) 2e+03 2e+03)
          (Utilities|Time|ClearandInvalidateTimerbyHandle (stale Input|EnhancedActionEvents|EnhancedInputActionIA_JumpIW _returnvalue)))))))

(event Input|EnhancedActionEvents|EnhancedInputActionIA_LookIW
  (params (ActionValue :type Vector%202D%20Structure) (ElapsedSeconds :type Float%20%28double-precision%29) (TriggeredSeconds :type Float%20%28double-precision%29) (InputAction :type Input%20Action%20Object%20Reference :default "/Game/Personnage/TheoInvisibleWoman/Input/IA_LookIW.IA_LookIW"))
  (Pawn|Input|AddControllerYawInput (Variables|Default|GetPlayer) (.x ActionValue))
  (Pawn|Input|AddControllerPitchInput (Variables|Default|GetPlayer) (.y ActionValue)))

(event Input|EnhancedActionEvents|EnhancedInputActionIA_MoveIW
  (params (ActionValue :type Vector%202D%20Structure) (ElapsedSeconds :type Float%20%28double-precision%29) (TriggeredSeconds :type Float%20%28double-precision%29) (InputAction :type Input%20Action%20Object%20Reference :default "/Game/Personnage/TheoInvisibleWoman/Input/IA_MoveIW.IA_MoveIW"))
  (bind _player (Variables|Default|GetPlayer))
  (bind _returnvalue (Pawn|GetControlRotation _player :!class /Script/Engine.Pawn))
  (Pawn|Input|AddMovementInput (Variables|Default|GetPlayer) (Math|Vector|GetRightVector (Math|Rotator|MakeRotator (.roll _returnvalue) 0.0 (.yaw _returnvalue))) (.x ActionValue) false)
  (Pawn|Input|AddMovementInput (Variables|Default|GetPlayer) (Math|Vector|GetForwardVector (Math|Rotator|MakeRotator 0.0 0.0 (.yaw (Pawn|GetControlRotation (Variables|Default|GetPlayer) :!class /Script/Engine.Pawn)))) (.y ActionValue) false))

(event Input|EnhancedActionEvents|EnhancedInputActionIA_JumpIW
  (params (ActionValue :type Boolean) (ElapsedSeconds :type Float%20%28double-precision%29) (TriggeredSeconds :type Float%20%28double-precision%29) (InputAction :type Input%20Action%20Object%20Reference :default "/Game/Personnage/TheoInvisibleWoman/Input/IA_JumpIW.IA_JumpIW"))
  (:Started
    (Character|Jump (Variables|Default|GetPlayer))
    (bind _returnvalue (Utilities|Time|SetTimerbyEvent (EventDispatchers|CreateEvent :!event Custom|JumpShake) (Utilities|Time|GetWorldDeltaSeconds) true)))
  (:Canceled
    (Character|StopJumping (Variables|Default|GetPlayer) :!label _label))
  (:Completed
    (goto _label)))

(event EventBeginPlay
  (bind _ascharacter (Utilities|Casting|CastToCharacter (Components|GetOwner)))
  (Variables|Default|SetPlayer _ascharacter))