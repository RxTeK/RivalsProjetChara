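; BP_InvisibleWoman is the player-controlled Invisible Woman character, handling basic movement, look and jump.
; On BeginPlay it adds the IMC_InvisibleWoman mapping context and creates the WBP_HUD widget on the player screen.
; Enhanced Input actions drive controller yaw and pitch, jumping, and movement relative to control rotation, with pitch zeroed to keep forward movement level.
; No invisibility or other ability logic is present.
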(event Input|EnhancedActionEvents|EnhancedInputActionIA_LookIW
  (params (ActionValue :type Vector%202D%20Structure) (ElapsedSeconds :type Float%20%28double-precision%29) (TriggeredSeconds :type Float%20%28double-precision%29) (InputAction :type Input%20Action%20Object%20Reference :default "/Game/Personnage/TheoInvisibleWoman/Input/IA_LookIW.IA_LookIW"))
  (Pawn|Input|AddControllerYawInput (.x ActionValue))
  (Pawn|Input|AddControllerPitchInput (.y ActionValue)))

(event Input|EnhancedActionEvents|EnhancedInputActionIA_MoveIW
  (params (ActionValue :type Vector%202D%20Structure) (ElapsedSeconds :type Float%20%28double-precision%29) (TriggeredSeconds :type Float%20%28double-precision%29) (InputAction :type Input%20Action%20Object%20Reference :default "/Game/Personnage/TheoInvisibleWoman/Input/IA_MoveIW.IA_MoveIW"))
  (bind _returnvalue (Pawn|GetControlRotation :!class /Script/Engine.Pawn))
  (Pawn|Input|AddMovementInput (Math|Vector|GetRightVector (Math|Rotator|MakeRotator (.roll _returnvalue) 0.0 (.yaw _returnvalue))) (.x ActionValue) false)
  (Pawn|Input|AddMovementInput (Math|Vector|GetForwardVector (Math|Rotator|MakeRotator 0.0 0.0 (.yaw (Pawn|GetControlRotation :!class /Script/Engine.Pawn)))) (.y ActionValue) false))

(event Input|EnhancedActionEvents|EnhancedInputActionIA_JumpIW
  (params (ActionValue :type Boolean) (ElapsedSeconds :type Float%20%28double-precision%29) (TriggeredSeconds :type Float%20%28double-precision%29) (InputAction :type Input%20Action%20Object%20Reference :default "/Game/Personnage/TheoInvisibleWoman/Input/IA_JumpIW.IA_JumpIW"))
  (:Started
    (Character|Jump))
  (:Canceled
    (Character|StopJumping :!label _label))
  (:Completed
    (goto _label)))

(event EventBeginPlay
  (bind _asplayer_controller (Utilities|Casting|CastToPlayerController (Pawn|GetController)))
  (Utilities|IsValid (PlayerController|LocalPlayerSubsystems|GetEnhancedInputLocalPlayerSubsystem _asplayer_controller)
    (:Is%20Valid
      (Input|AddMappingContext (PlayerController|LocalPlayerSubsystems|GetEnhancedInputLocalPlayerSubsystem _asplayer_controller) "/Game/Personnage/TheoInvisibleWoman/Input/IMC_InvisibleWoman.IMC_InvisibleWoman" 0 "(bIgnoreAllPressedKeysUntilRelease=True,bForceImmediately=False,bNotifyUserSettings=False)")
      (bind _returnvalue (UserInterface|CreateWidget "/Game/Personnage/TheoInvisibleWoman/Blueprint/HUD/WBP_HUD.WBP_HUD_C"))
      (UserInterface|Viewport|AddtoPlayerScreen _returnvalue))))

(fn ConstructionScript)