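; BP_grenade is the Punisher's grenade actor, which flies along a path supplied by the player pawn.
; On BeginPlay it copies BP_Punisher's ArrayLocation points into InterpToMovement as absolute control points and activates it.
; Each tick a small sphere trace checks for contact.
; The first hit runs a large debug-drawn blast-radius trace, whose result is unused, then destroys the actor after a short delay.
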(event EventBeginPlay
  (bind _interptomovement (Variables|Default|GetInterpToMovement))
  (Utilities|FlowControl|Sequence
    (:then_0
      (bind _asbp_punisher (Utilities|Casting|CastToBP_Punisher (Game|Player|GetPlayerPawn 0)))
      (Variables|Default|SetPunisherREF _asbp_punisher))
    (:then_1
      (for (_ _array_index) (Variables|/Game/Punisher/Bp/BP_Punisher.BP_Punisher_C|GetArrayLocation (Variables|Default|GetPunisherREF))
        (Class|InterptoMovementComponent|AddControlPointPosition _interptomovement (Utilities|Array|Get(acopy) (Variables|/Game/Punisher/Bp/BP_Punisher.BP_Punisher_C|GetArrayLocation (Variables|Default|GetPunisherREF)) _array_index) false))
      (Class|InterptoMovementComponent|FinaliseControlPoints _interptomovement)
      (Components|Activation|Activate (Variables|Default|GetInterpToMovement) false))))

(event EventTick
  (params (DeltaSeconds :type Float%20%28single-precision%29))
  (bind _sphere (Variables|Default|GetSphere))
  (bind _sphere_2 (Variables|Default|GetSphere))
  (bind _returnvalue (Transformation|GetWorldLocation _sphere))
  (bind _returnvalue_2 (Transformation|GetWorldLocation _sphere_2))
  (bind _returnvalue_3 (Collision|SphereTraceByChannel _returnvalue_2 _returnvalue_2 15.0 "TraceTypeQuery1" false 0 "ForDuration"))
  (if _returnvalue_3
    (Utilities|FlowControl|DoOnce false
      (:Completed
        (Collision|SphereTraceByChannel _returnvalue _returnvalue 5e+02 "TraceTypeQuery1" false 0 "ForDuration")
        (Utilities|FlowControl|Delay 2.0)
        (Actor|DestroyActor)))))

(fn ConstructionScript)