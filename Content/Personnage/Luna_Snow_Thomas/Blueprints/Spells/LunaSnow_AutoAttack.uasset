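; Luna Snow's auto-attack component, a hold-to-fire primary attack built as a hitscan prototype for its BP_Player owner.
; Holding primary click loops AutoAttack every half second, and release stops it, with a short delay before re-arming.
; Each attack starts a fast timer on "tierre", a name unlike the Tir function that holds the three-shot burst logic.
; Tir line-traces from the follow camera with debug drawing and no hit handling.
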(event Custom|AutoAttack
  ;[0.3121 0.03384 0.4566] LineTrace Auto
  (Variables|Default|SetCount 0)
  (bind _returnvalue (Utilities|Time|SetTimerbyFunctionName 0 "tierre" 0.1 true false -0.1))
  (Variables|Default|SetTire _returnvalue))

(event Custom|DelayAuto
  ;[0.3121 0.03384 0.4566] LineTrace Auto
  (Variables|Default|SetREAuto true))

(event Input|EnhancedActionEvents|EnhancedInputActionIA_Primary_Click
  (params (ActionValue :type Boolean) (ElapsedSeconds :type Float%20%28double-precision%29) (TriggeredSeconds :type Float%20%28double-precision%29) (InputAction :type Input%20Action%20Object%20Reference :default "/Game/Personnage/Cyril_Mantis/Input/IA_Primary_Click.IA_Primary_Click"))
  ;[0.3121 0.03384 0.4566] LineTrace Auto
  (:Started
    (if (Variables|Default|GetREAuto)
      (Variables|Default|SetREAuto false)
      (bind _returnvalue (Utilities|Time|SetTimerbyEvent (delegate Custom|AutoAttack) 0.5 true false -0.5))
      (Variables|Default|SetTimer _returnvalue)))
  (:Completed
    (if (Utilities|Time|IsValidTimerHandle (Variables|Default|GetTimer))
      (Utilities|Time|ClearandInvalidateTimerbyHandle (Variables|Default|GetTimer))
      (Utilities|Time|SetTimerbyEvent (delegate Custom|DelayAuto) 0.5))))

(event EventBeginPlay
  ;[0.3121 0.03384 0.4566] LineTrace Auto
  (bind _asbp_player (Utilities|Casting|CastToBP_Player (Components|GetOwner)))
  (Variables|Default|SetAs%20BP%20Luna%20Snow _asbp_player))

(fn Tir
  (bind _as_bp_luna_snow (Variables|Default|GetAs%20BP%20Luna%20Snow))
  (bind _followcamera (Variables|/Game/Personnage/ALL/BP_Player.BP_Player_C|GetFollowCamera _as_bp_luna_snow))
  (bind _returnvalue (Transformation|GetWorldLocation _followcamera))
  (Collision|LineTraceByChannel _returnvalue (+ _returnvalue (* (Math|Vector|GetForwardVector _followcamera) 1000000000)) "TraceTypeQuery1" false 0 "ForDuration")
  (if (>= (Variables|Default|GetCount) 2)
    (Utilities|Time|ClearandInvalidateTimerbyHandle (Variables|Default|GetTire))
    (else
      (Math|Integer|IncrementInt (Variables|Default|GetCount)))))