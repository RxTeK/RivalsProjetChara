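; Luna Snow's secondary-click spell component, which fires a BP_Projectile_LunaSnow from the owning player's ProjectilePoint.
; On input, a visibility line trace along that point's forward vector picks the target, and the projectile spawns facing the hit or trace end.
; A one-second timer handle acts as the cooldown, blocking recasts until it is cleared.
; Debug trace drawing and a print remain, and the ClicDroitSpell function is empty.
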(event Custom|Spell1
  (Utilities|Time|ClearandInvalidateTimerbyHandle (Variables|Default|GetTimer)))

(event Input|EnhancedActionEvents|EnhancedInputActionIA_Secondary_Click
  (params (ActionValue :type Boolean) (ElapsedSeconds :type Float%20%28double-precision%29) (TriggeredSeconds :type Float%20%28double-precision%29) (InputAction :type Input%20Action%20Object%20Reference :default "/Game/Personnage/Cyril_Mantis/Input/IA_Secondary_Click.IA_Secondary_Click"))
  (bind _as_bp_luna_snow (Variables|Default|GetAs%20BP%20Luna%20Snow))
  (bind _projectilepoint (Variables|/Game/Personnage/ALL/BP_Player.BP_Player_C|GetProjectilePoint _as_bp_luna_snow))
  (bind _returnvalue (Transformation|GetWorldLocation _projectilepoint))
  (:Started
    (if (not (Utilities|Time|IsValidTimerHandle (Variables|Default|GetTimer)))
      (bind (_outhit _returnvalue_2) (Collision|LineTraceByChannel _returnvalue (+ _returnvalue (* (Math|Vector|GetForwardVector _projectilepoint) 1000000000)) "TraceTypeQuery1" false 0 "ForDuration"))
      (Game|SpawnActorfromClass "/Game/Personnage/Luna_Snow_Thomas/Blueprints/BP_Projectile_LunaSnow.BP_Projectile_LunaSnow_C" (Math|Transform|MakeTransform _returnvalue (Math|Conversions|RotationFromXVector (Math|Vector|GetUnitDirection(Vector) _returnvalue (select _returnvalue_2 (.Location (Collision|BreakHitResult _outhit)) (.TraceEnd (Collision|BreakHitResult _outhit))))) "1.000000,1.000000,1.000000") "Undefined" "MultiplyWithRoot" 0 0)
      (bind _returnvalue_3 (Utilities|Time|SetTimerbyEvent (delegate Custom|Spell1) 1.0))
      (Variables|Default|SetTimer _returnvalue_3)
      (Development|PrintString "ClicDroit"))))

(event EventBeginPlay
  (bind _asbp_player (Utilities|Casting|CastToBP_Player (Components|GetOwner)))
  (Variables|Default|SetAs%20BP%20Luna%20Snow _asbp_player))

(fn ClicDroitSpell)