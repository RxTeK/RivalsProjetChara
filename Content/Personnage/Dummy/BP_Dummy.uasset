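; Configurable training dummy with a health bar, tinted red as an enemy or blue as an ally.
; BeginPlay picks one flag-driven behavior: timed switch to flying with a timeline rise, back-and-forth timeline patrol, or repeated BP_DummyShoot spawning.
; Damage updates HP and the widget, optionally starting a timer that restores full health.
; Tick always shows enemy bars, but shows ally bars only when the player is a healer.
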(event Custom|ResetLife
  ;[0.4434 1 0] Regen
  (Variables|Default|SetStat (Utilities|Struct|MakeBaseStat (.maxhp (Variables|Default|GetStat)) (.maxhp (Variables|Default|GetStat)) (.movespeed (Variables|Default|GetStat)) (.energy (Variables|Default|GetStat)) (.energymax (Variables|Default|GetStat))))
  (Default|SetHP (Variables|Default|GetWidget%20REF) (.hp (Variables|Default|GetStat)) (.maxhp (Variables|Default|GetStat))))

(event Custom|Flying?
  (bind _returnvalue (Transformation|GetActorLocation))
  ;[1 0.2204 0] Fly
  (if (not (Utilities|Enum|Equal(Enum) (Variables|/Script/Engine.CharacterMovementComponent|GetMovementMode (Variables|Character|GetCharacterMovement)) "MOVE_Flying"))
    (Pawn|Components|CharacterMovement|SetMovementMode (Variables|Character|GetCharacterMovement) "MOVE_Flying" 0)
    (Variables|Default|SetReturn%20Value%20Z (.z (Transformation|GetActorLocation)))
    (bind _newtrack_0 (Timeline|Timeline_0 PlayFromStart)
      (:Update
        (Transformation|SetActorLocation (Math|Vector|MakeVector (.x _returnvalue) (.y _returnvalue) (+ (Variables|Default|GetReturn%20Value%20Z) (* _newtrack_0 (Variables|Default|GetFlyPosition)))) false false)))))

(event Custom|Spawn
  (bind _self self)
  (bind _returnvalue (Transformation|GetActorLocation _self))
  (bind _returnvalue_2 (Transformation|GetActorForwardVector _self))
  (bind _returnvalue_3 (* _returnvalue_2 1.4e+02))
  (bind _returnvalue_4 (+ _returnvalue _returnvalue_3))
  ;[0 0.4163 1] Shoot
  (Game|SpawnActorfromClass "/Game/Personnage/Dummy/BP_DummyShoot.BP_DummyShoot_C" (Math|Transform|MakeTransform (Math|Vector|MakeVector (.x _returnvalue_4) (.y _returnvalue_4) (+ (.z _returnvalue_4) 4e+01)) (Math|Conversions|RotationFromXVector (Transformation|GetActorForwardVector)) "1.000000,1.000000,1.000000") "Undefined" "MultiplyWithRoot" 0 0))

(event Custom|Change
  (bind _returnvalue (Transformation|GetActorLocation))
  (if (Variables|Default|GetReversed)
    ;[1 0 0.5923] Movement
    (Variables|Default|SetReverseValue -1e+01)
    (Variables|Default|SetReversed false)
    (bind _newtrack_0 (Timeline|Timeline PlayFromStart)
      (:Update
        (Transformation|SetActorLocation (Math|Vector|MakeVector (+ (* _newtrack_0 (Variables|Default|GetReverseValue)) (.x _returnvalue)) (.y _returnvalue) (.z _returnvalue)) false false))
      (:Finished
        (Transformation|SetActorRotation (Math|Rotator|MakeRotator 0.0 0.0 (+ (.yaw (Transformation|GetActorRotation)) 1.8e+02)))
        (CallFunction|Change)))
    (else
      (Variables|Default|SetReverseValue 1e+01)
      (Variables|Default|SetReversed true)
      (Timeline|Timeline ReverseFromEnd))))

(event EventBeginPlay
  (bind _returnvalue (Transformation|GetActorLocation))
  (bind _stat (Variables|Default|GetStat))
  ;[0.7999 0.8475 1] BeginPlay
  (bind _aswbp_life_bar (Utilities|Casting|CastToWBP_LifeBar (UserInterface|GetWidget (Variables|Default|GetWidget))))
  (bind _output_get (Variables|Default|SetWidget%20REF _aswbp_life_bar))
  (Default|SetHP _output_get (.hp _stat) (.maxhp _stat))
  (Utilities|FlowControl|Sequence
    (:then_0
      (bind _asbp_player (Utilities|Casting|CastToBP_Player (Game|GetPlayerCharacter 0)))
      (Variables|Default|SetAs%20BP%20Player _asbp_player))
    (:then_1
      (if (Variables|Default|GetFlying)
        ;[1 0.2204 0] Fly
        (Utilities|Time|SetTimerbyEvent (delegate Custom|Flying?) (Variables|Default|GetTimeBetweenFly) true false -8.0)
        (elif (Variables|Default|GetMoving)
          (Components|Animation|PlayAnimation (Variables|Character|GetMesh) "/Game/Personnage/ScarletWitch/Export/RetargetAnim/SWAnimScarletWitch_SK_1038_1038001_Run_Fwd_C_Montage.SWAnimScarletWitch_SK_1038_1038001_Run_Fwd_C_Montage" true)
          (if (Variables|Default|GetReversed)
            ;[1 0 0.5923] Movement
            (Variables|Default|SetReverseValue -1e+01)
            (Variables|Default|SetReversed false)
            (bind _newtrack_0 (Timeline|Timeline PlayFromStart)
              (:Update
                (Transformation|SetActorLocation (Math|Vector|MakeVector (+ (* _newtrack_0 (Variables|Default|GetReverseValue)) (.x _returnvalue)) (.y _returnvalue) (.z _returnvalue)) false false))
              (:Finished
                (Transformation|SetActorRotation (Math|Rotator|MakeRotator 0.0 0.0 (+ (.yaw (Transformation|GetActorRotation)) 1.8e+02)))
                (CallFunction|Change)))
            (else
              (Variables|Default|SetReverseValue 1e+01)
              (Variables|Default|SetReversed true)
              (Timeline|Timeline ReverseFromEnd)))
          (elif (Variables|Default|GetShoot)
            (Utilities|Time|SetTimerbyEvent (delegate Custom|Spawn) 1.0 true)))))))

(event Game|Damage|EventAnyDamage
  (params (Damage :type Float%20%28single-precision%29) (DamageType :type Damage%20Type%20Object%20Reference) (InstigatedBy :type Controller%20Object%20Reference) (DamageCauser :type Actor%20Object%20Reference))
  ;[0.3698 0.004212 0] Apply Damage
  (Utilities|FlowControl|Sequence
    (:then_0
      (Variables|Default|SetStat (Utilities|Struct|MakeBaseStat (- (.HP (Utilities|Struct|BreakBaseStat (Variables|Default|GetStat))) Damage) (.MaxHP (Utilities|Struct|BreakBaseStat (Variables|Default|GetStat))) (.MoveSpeed (Utilities|Struct|BreakBaseStat (Variables|Default|GetStat)))))
      (Default|SetHP (Variables|Default|GetWidget%20REF) (.hp (Variables|Default|GetStat)) (.maxhp (Variables|Default|GetStat))))
    (:then_1
      (if (Variables|Default|GetCanRegen)
        ;[0.4434 1 0] Regen
        (Utilities|Time|SetTimerbyEvent (delegate Custom|ResetLife) (Variables|Default|GetTime%20between%20Regen))))))

(event EventTick
  (params (DeltaSeconds :type Float%20%28single-precision%29))
  ;[0 1 0.08472] Life Bar Visibility
  (Utilities|IsValid (Variables|Default|GetAs%20BP%20Player)
    (:Is%20Valid
      (switch Utilities|FlowControl|Switch|SwitchonE_DummyType (Variables|Default|GetDummyType)
        (:NewEnumerator0
          (Rendering|SetVisibility (Variables|Default|GetWidget) true false))
        (:NewEnumerator1
          (if (Variables|/Game/Personnage/ALL/BP_Player.BP_Player_C|GetIsHealer (Variables|Default|GetAs%20BP%20Player))
            (Rendering|SetVisibility (Variables|Default|GetWidget) true false)
            (else
              (Rendering|SetVisibility (Variables|Default|GetWidget) false false))))))))

(fn ConstructionScript
  (bind _mesh (Variables|Character|GetMesh))
  (switch Utilities|FlowControl|Switch|SwitchonE_DummyType (Variables|Default|GetDummyType)
    (:NewEnumerator0
      (Rendering|Material|SetVectorParameterValueonMaterials _mesh "Tint" "1.000000,0.000000,0.000000"))
    (:NewEnumerator1
      (Rendering|Material|SetVectorParameterValueonMaterials _mesh "Tint" "0.000000,0.000000,1.000000"))))