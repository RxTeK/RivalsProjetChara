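; BP_DummyShoot is an actor, apparently a shot fired by BP_Dummy, that damages characters it touches.
; On BeginPlay it casts its instigator to BP_Dummy and caches the reference.
; When its box begins overlapping a Character and that dummy's DummyType is Ennemy, it applies fixed damage and destroys itself.
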(event OnComponentBeginOverlap(Box)
  (params (OverlappedComponent :type Primitive%20Component%20Object%20Reference) (OtherActor :type Actor%20Object%20Reference) (OtherComp :type Primitive%20Component%20Object%20Reference) (OtherBodyIndex :type Integer) (bFromSweep :type Boolean) (SweepResult :type Hit%20Result%20Structure%20%28by%20ref%29))
  (bind (_ascharacter _bsuccess) (Utilities|Casting|CastToCharacter OtherActor))
  (if _bsuccess
    (switch Utilities|FlowControl|Switch|SwitchonE_DummyType (Variables|/Game/Personnage/Dummy/BP_Dummy.BP_Dummy_C|GetDummyType (Variables|Default|GetAs%20BP%20Dummy))
      (:NewEnumerator0
        (Game|Damage|ApplyDamage _ascharacter 25.0 0 0)
        (Actor|DestroyActor)))))

(event EventBeginPlay
  (bind _asbp_dummy (Utilities|Casting|CastToBP_Dummy (Game|GetInstigator)))
  (Variables|Default|SetAs%20BP%20Dummy _asbp_dummy))

(fn ConstructionScript)