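; Ability logic for BP_HawkEyes that charges and fires arrows, caching its owner on BeginPlay.
; ChargeArrow raises a capped ArrowStrong value and prints it.
; When Triple is true, ShootArrow clears the charge timer, traces from the camera, spawns a BP_Arrow aimed at the hit or trace end with that charge, then resets it.
; A three-arrow loop is unconnected, and a false Triple does nothing.
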(event Custom|ChargeArrow
  (bind _output_get (Variables|Default|SetArrowStrong (Math|Float|Clamp(Float) (+ (Variables|Default|GetArrowStrong) 3.0) 0.0 1e+02)))
  (Development|PrintString (Utilities|String|ToString(Float) _output_get) true true "(R=0.210475,G=1.000000,B=0.000000,A=1.000000)" 0.0))

(event Custom|ShootArrow
  (params (Triple :type Boolean))
  (bind _hawk_ref (Variables|Default|GetHawk_Ref))
  (bind _hawk_ref_2 (Variables|Default|GetHawk_Ref))
  (bind _spawnarrow (Variables|/Game/MaximeHawkEye/Blueprint/BP_HawkEyes.BP_HawkEyes_C|GetSpawnArrow _hawk_ref_2))
  (bind _followcamera (Variables|/Game/MaximeHawkEye/Blueprint/BP_HawkEyes.BP_HawkEyes_C|GetFollowCamera _hawk_ref))
  (bind _returnvalue (Transformation|GetWorldLocation _followcamera))
  (bind _returnvalue_2 (Transformation|GetWorldLocation _spawnarrow))
  (if Triple
    (Utilities|Time|ClearandInvalidateTimerbyHandle (Variables|/Game/MaximeHawkEye/Blueprint/BP_HawkEyes.BP_HawkEyes_C|GetChargeArrowTH (Variables|Default|GetHawk_Ref)))
    (bind (_outhit _returnvalue_3) (Collision|LineTraceByChannel _returnvalue (+ _returnvalue (* (Math|Vector|GetForwardVector _followcamera) 4e+03)) "TraceTypeQuery1" false 0 "Persistent"))
    (Game|SpawnActorfromClass "/Game/MaximeHawkEye/Blueprint/BP_Arrow.BP_Arrow_C" (Math|Transform|MakeTransform _returnvalue_2 (Math|Rotator|FindLookatRotation _returnvalue_2 (select _returnvalue_3 (.Location (Collision|BreakHitResult _outhit)) (.TraceEnd (Collision|BreakHitResult _outhit)))) "1.000000,1.000000,1.000000") "Undefined" "MultiplyWithRoot" 0 (Variables|Default|GetArrowStrong) 0.0 0)
    (Variables|Default|SetArrowStrong 0.0)))

(event EventBeginPlay
  (bind _asbp_hawk_eyes (Utilities|Casting|CastToBP_HawkEyes (Components|GetOwner)))
  (Variables|Default|SetHawk_Ref _asbp_hawk_eyes))

(event EventTick
  (params (DeltaSeconds :type Float%20%28single-precision%29)))