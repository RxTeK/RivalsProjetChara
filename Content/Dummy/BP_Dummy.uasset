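; BP_Dummy is a dummy actor that can be configured as an enemy or an ally and shows its health on a life bar widget.
; The construction script tints the skeletal mesh red for enemies or blue for allies, based on DummyType.
; On BeginPlay it caches the WBP_LifeBar from its widget component and sets it to the current and maximum HP from Stat.
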(event EventBeginPlay
  (bind _stat (Variables|Default|GetStat))
  (bind _aswbp_life_bar (Utilities|Casting|CastToWBP_LifeBar (UserInterface|GetWidget (Variables|Default|GetWidget))))
  (bind _output_get (Variables|Default|SetWidget%20REF _aswbp_life_bar))
  (Default|SetHP _output_get (.hp _stat) (.maxhp _stat)))

(event Collision|EventActorBeginOverlap
  (params (OtherActor :type Actor%20Object%20Reference)))

(event EventTick
  (params (DeltaSeconds :type Float%20%28single-precision%29)))

(fn ConstructionScript
  (switch Utilities|FlowControl|Switch|SwitchonE_DummyType (Variables|Default|GetDummyType)
    (:NewEnumerator0
      (Rendering|Material|SetVectorParameterValueonMaterials (Variables|Default|GetSkeletalMesh) "Tint" "1.000000,0.000000,0.000000"))
    (:NewEnumerator1
      (Rendering|Material|SetVectorParameterValueonMaterials (Variables|Default|GetSkeletalMesh) "Tint" "0.000000,0.000000,1.000000"))))